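; Shooter HUD that owns and drives the player state, inventory, dynamic crosshair and damage indicator widgets.
; BeginPlay creates the first three, while the damage indicator appears on demand with the hit location.
; Request events forward crosshair, inventory, health, armor, boost and ammo updates to those widgets, normalizing stat values.
; Inventory toggling switches input mode and mouse cursor, with a short delay lock against rapid re-toggling.
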(event `self.ReceiveBeginPlay`
  ;[1 1 1] Begin Play
  (`self.Create_Player_State`)
  (`self.Create_Inventory_Layout`)
  (`self.Create_Dynamic_Crosshair`))

(event `self.Create_Dynamic_Crosshair`
  ;[1 1 1] Dynamic Crosshair Events
  (`/Engine/EditorBlueprintResources/StandardMacros.IsValid` (`self.CrosshairReference`)
    (:`Is Valid`
      _)
    (:`Is Not Valid`
      (bind _returnvalue (`|CreateWidget` "/Game/UltimateShooterKit/UserInterface/Widget_DynamicCrosshair.Widget_DynamicCrosshair_C" (`self.GetOwningPlayerController`)))
      (set `self.CrosshairReference` _returnvalue)))
  (`UserWidget.AddToViewport` (`self.CrosshairReference`) 0))

(event `self.Toggle_Crosshair`
  (params (`Visible?` :type Boolean))
  ;[1 1 1] Dynamic Crosshair Events
  (`/Game/UltimateShooterKit/UserInterface/Widget_DynamicCrosshair.Toggle_Crosshair` (`self.CrosshairReference`) `Visible?`))

(event `self.On_Hit_Crosshair`
  ;[1 1 1] Dynamic Crosshair Events
  (`/Game/UltimateShooterKit/UserInterface/Widget_DynamicCrosshair.On_Hit` (`self.CrosshairReference`)))

(event `self.Update_Crosshair_Spread`
  (params (SpreadAmount :type "Float (single-precision)") (InterpSpeed :type "Float (single-precision)"))
  ;[1 1 1] Dynamic Crosshair Events
  (`/Game/UltimateShooterKit/UserInterface/Widget_DynamicCrosshair.Update_Crosshair_Spread` (`self.CrosshairReference`) SpreadAmount InterpSpeed))

(event `self.Create_Damage_Indicator`
  (params (HitLocation :type "Vector Structure"))
  (bind _damageindicatorreference (`self.DamageIndicatorReference`))
  ;[1 1 1] Damage Indicator
  (`/Engine/EditorBlueprintResources/StandardMacros.IsValid` (`self.DamageIndicatorReference`)
    (:`Is Valid`
      _)
    (:`Is Not Valid`
      (bind _returnvalue (`|CreateWidget` "/Game/UltimateShooterKit/UserInterface/Widget_DamageIndicator.Widget_DamageIndicator_C" (`self.GetOwningPlayerController`)))
      (set `self.DamageIndicatorReference` _returnvalue)))
  (if (not (`Widget.IsInViewport` _damageindicatorreference))
    (`UserWidget.AddToViewport` _damageindicatorreference 0))
  (`/Game/UltimateShooterKit/UserInterface/Widget_DamageIndicator.Update_Hit_Location` (`self.DamageIndicatorReference`) HitLocation 3.0))

(event `Create_Inventory_Layout`
  ;[1 1 1] Create Inventory Widget
  (`/Engine/EditorBlueprintResources/StandardMacros.IsValid` (`self.InventoryLayoutReference`)
    (:`Is Valid`
      _)
    (:`Is Not Valid`
      (bind _returnvalue (`|CreateWidget` "/Game/UltimateShooterKit/UserInterface/Widget_InventoryLayout.Widget_InventoryLayout_C" (`self.GetOwningPlayerController`)))
      (set `self.InventoryLayoutReference` _returnvalue)))
  (`UserWidget.AddToViewport` (`self.InventoryLayoutReference`) 0))

(event `self.Request_Refresh_Weapons`
  ;[1 1 1] Create Inventory Widget
  (`/Game/UltimateShooterKit/UserInterface/Widget_InventoryLayout.Refresh_Weapons` (`self.InventoryLayoutReference`)))

(event `self.Request_Update_Inventory_Size`
  (params (NewSize :type "Float (single-precision)") (InMax :type "Float (single-precision)"))
  ;[1 1 1] Create Inventory Widget
  (`/Game/UltimateShooterKit/UserInterface/Widget_InventoryLayout.Update_Inventory_Size` (`self.InventoryLayoutReference`) NewSize InMax))

(event `self.Request_Refresh_Consumables`
  ;[1 1 1] Create Inventory Widget
  (`/Game/UltimateShooterKit/UserInterface/Widget_InventoryLayout.Refresh_Inventory_Items` (`self.InventoryLayoutReference`)))

(event `self.Request_Toggle_Inventory`
  (bind (_returnvalue_x _returnvalue_y) (`KismetMathLibrary.BreakVector2D` (`WidgetLayoutLibrary.GetViewportSize`)))
  ;[1 1 1] Create Inventory Widget
  (if (`self.CanToggleInventory?`)
    (set `self.CanToggleInventory?` false)
    (`|ExecutionSequence`
      (:`then_0`
        (set `self.IsInventoryOpened?` (not (`self.IsInventoryOpened?`)))
        (`/Game/UltimateShooterKit/UserInterface/Widget_InventoryLayout.Toggle_Inventory` (`self.InventoryLayoutReference`) (`self.IsInventoryOpened?`))
        (if (`self.IsInventoryOpened?`)
          (`WidgetBlueprintLibrary.SetInputMode_GameAndUIEx` (`self.GetOwningPlayerController`) (`self.InventoryLayoutReference`) "LockAlways" false)
          (set `PlayerController.bShowMouseCursor` true (`self.GetOwningPlayerController`))
          (`PlayerController.SetMouseLocation` (`self.GetOwningPlayerController`) (`KismetMathLibrary.FTrunc` (/ _returnvalue_x 1.15)) (`KismetMathLibrary.FTrunc` (/ _returnvalue_y 2.0)))
          (else
            (`WidgetBlueprintLibrary.SetInputMode_GameOnly` (`self.GetOwningPlayerController`))
            (set `PlayerController.bShowMouseCursor` false (`self.GetOwningPlayerController`)))))
      (:`then_1`
        (`KismetSystemLibrary.Delay` 0.5)
        (set `self.CanToggleInventory?` true)))))

(event `Create_Player_State`
  ;[1 1 1] Player State Widget
  (`/Engine/EditorBlueprintResources/StandardMacros.IsValid` (`self.PlayerStateReference`)
    (:`Is Valid`
      _)
    (:`Is Not Valid`
      (bind _returnvalue (`|CreateWidget` "/Game/UltimateShooterKit/UserInterface/Widget_PlayerState.Widget_PlayerState_C" (`self.GetOwningPlayerController`)))
      (set `self.PlayerStateReference` _returnvalue)))
  (`UserWidget.AddToViewport` (`self.PlayerStateReference`) 0))

(event `self.Request_Update_Health`
  (params (NewHealthValue :type "Float (single-precision)") (InMaxHealth :type "Float (single-precision)") (InTime :type Boolean))
  ;[1 1 1] Player State Widget
  (`/Game/UltimateShooterKit/UserInterface/Widget_PlayerState.Update_Health` (`self.PlayerStateReference`) NewHealthValue (`KismetMathLibrary.NormalizeToRange` NewHealthValue 0.0 InMaxHealth) InTime))

(event `self.Request_Update_Armor`
  (params (NewArmorValue :type "Float (single-precision)") (InMaxArmor :type "Float (single-precision)"))
  ;[1 1 1] Player State Widget
  (`/Game/UltimateShooterKit/UserInterface/Widget_PlayerState.Update_Armor` (`self.PlayerStateReference`) NewArmorValue (`KismetMathLibrary.NormalizeToRange` NewArmorValue 0.0 InMaxArmor)))

(event `self.Request_Update_Boost`
  (params (NewBoostValue :type "Float (single-precision)") (InMaxBoost :type "Float (single-precision)"))
  ;[1 1 1] Player State Widget
  (`/Game/UltimateShooterKit/UserInterface/Widget_PlayerState.Update_Boost` (`self.PlayerStateReference`) NewBoostValue (`KismetMathLibrary.NormalizeToRange` NewBoostValue 0.0 InMaxBoost)))

(event `self.Request_Update_Ammunition_Info`
  (params (`Visible?` :type Boolean) (Current :type Integer) (Total :type Integer))
  ;[1 1 1] Player State Widget
  (`/Game/UltimateShooterKit/UserInterface/Widget_PlayerState.Update_Ammunition_Info` (`self.PlayerStateReference`) `Visible?` Current Total))

(fn `Get_Is_Inventory_Opened`
  (returns (ReturnValue :type Boolean))
  (return (`self.IsInventoryOpened?`)))

(fn `UserConstructionScript`)