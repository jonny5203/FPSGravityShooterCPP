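; BP_ShooterController is the player controller for the Ultimate Shooter Kit, linking the possessed pawn to inventory and interaction state.
; On possession it passes the new pawn to its InventoryComponent, and pressing Tab asks the HUD to toggle the inventory.
; It also exposes the inventory component and stores the currently available interaction type through simple getter and update functions.
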(event `Key|Tab`
  (params (Key :type "Key Structure"))
  (:`Pressed`
    (message `/Game/UltimateShooterKit/Blueprints/Data/Interfaces/BP_HUDInterface.Request_Toggle_Inventory` (`self.GetHUD`))))

(event `self.ReceivePossess`
  (params (PossessedPawn :type "Pawn Object Reference"))
  (`/Game/UltimateShooterKit/Blueprints/Components/Component_Inventory.On_Possess` (`self.InventoryComponent`) PossessedPawn))

(fn `Get_InventoryComponent`
  (returns (InventoryComponent :type "/Game/UltimateShooterKit/Blueprints/Components/Component_Inventory Object Reference"))
  (return (`self.InventoryComponent`)))

(fn `GetCurrentInteractionType`
  (returns (ReturnValue :type "/Game/UltimateShooterKit/Blueprints/Data/Enumerations/Enum_InteractionType Enum"))
  (return (`self.AvailableInteractionType`)))

(fn `UpdateInteractionType`
  (params (NewInteractionType :type "/Game/UltimateShooterKit/Blueprints/Data/Enumerations/Enum_InteractionType Enum" :default "NewEnumerator0"))
  (returns (Success :type Boolean))
  (set `self.AvailableInteractionType` NewInteractionType)
  (return true))

(fn `UserConstructionScript`)