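; Player camera manager for the shooter character, handling first- and third-person views, aiming, ADS and shoulder swapping, including temporary lean swaps.
; BlueprintUpdateCamera pivots on the mesh's "Camera" socket with clamped Z smoothing, follows control rotation and sphere-traces against obstructions.
; State changes start a looping timer that blends camera offset and FOV along a curve.
; Perspective and ADS transitions message the pawn to toggle its head mesh.
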(event `self.On_Aim_Down_Sights`
  (params (`IsADS?` :type Boolean) (TargetFOV :type "Float (single-precision)"))
  (bind _isaiming_ (`self.IsAiming?`))
  (bind ((`TPPCameraPosition_25_BC220C244C070F1D70C33A8CF2BBD23C` _tppcameraposition) (`TPPAimCameraPosition_28_7910E5814ED69593F5F18D98B478F38D` _tppaimcameraposition) (`TPPFOV_19_240B347A4EA971B806A7AB91D0A4BFC2` _tppfov) (`TPPAimFOV_31_0AC1E3BE4CBF932D997A9D82A9E3C815` _tppaimfov)) (break `/Game/UltimateShooterKit/Blueprints/Data/Structures/CameraStructs/Struct_CameraSettings` (select `bool` (`self.ShoulderSwitchedTemporary`) :`false` (`self.MakeCameraSettings`) :`true` (`self.MakeCustomCameraSettings` (`self.ShoulderOnLeft`)))))
  ;[1 1 1] Aim Down Sights
  (bind _output_get (set `self.IsADS?` `IsADS?`))
  (if _output_get
    (if (`self.IsFirstPerson?`)
      (`self.Start_Camera_Timer` (0.0 0.0 0.0) TargetFOV)
      (else
        (set `self.DesiredCameraPosition` (0.0 0.0 0.0))
        (message `/Game/UltimateShooterKit/Blueprints/Data/Interfaces/BP_PlayerPawnInterface.On_Perspective_Changed` (`self.GetOwningPawn`) true)
        (`self.Start_Camera_Timer` (0.0 0.0 0.0) TargetFOV)))
    (elif (`self.IsFirstPerson?`)
      (`self.Start_Camera_Timer` (0.0 0.0 0.0) (`.FPPFOV_21_D3A933C340CDC2D41FD20AA72C238C14` (break `/Game/UltimateShooterKit/Blueprints/Data/Structures/CameraStructs/Struct_CameraSettings` (`self.MakeCameraSettings`))))
      (else
        (`self.Start_Camera_Timer` (`KismetMathLibrary.SelectVector` _tppaimcameraposition _tppcameraposition _isaiming_) (`KismetMathLibrary.SelectFloat` _tppaimfov _tppfov _isaiming_))
        (message `/Game/UltimateShooterKit/Blueprints/Data/Interfaces/BP_PlayerPawnInterface.On_Perspective_Changed` (`self.GetOwningPawn`) false)))))

(event `self.ReceiveBeginPlay`
  ;[1 1 1] Reset Camera Settings On Begin Play
  (`self.Update_Camera_Settings` (`self.MakeCameraSettings`)))

(event `self.Update_Camera_Settings`
  (params (CameraSettings :type "/Game/UltimateShooterKit/Blueprints/Data/Structures/CameraStructs/Struct_CameraSettings Structure"))
  (bind ((`CameraOffsets_11_0328D19A495C535B37D20B8921B7AB1E` _cameraoffsets) (`CameraCurve_24_1FB4A9C044FCAE34558875BD1FC9BE8E` _cameracurve)) (break `/Game/UltimateShooterKit/Blueprints/Data/Structures/CameraStructs/Struct_CameraSettings` CameraSettings))
  (bind (_camerapivotoffset _cameraoffset) (break `/Game/UltimateShooterKit/Blueprints/Data/Structures/CameraStructs/Struct_DefaultCameraOffsets` _cameraoffsets))
  ;[1 1 1] Update Camera Settings
  (set `self.CameraPositionCurve` _cameracurve)
  (set `self.DefaultPivotOffset` _camerapivotoffset)
  (set `self.DefaultCameraOffset` _cameraoffset)
  (message `/Game/UltimateShooterKit/Blueprints/Data/Interfaces/BP_OverlayAnimBPInterface.Set_CameraOffset` (`self.GetOverlayAnimInstance` "ShooterOverlay") (+ (`self.DefaultPivotOffset`) (`self.DefaultCameraOffset`))))

(event `Start_Camera_Timer`
  (params (CameraLerpTarget :type "Vector Structure") (FOV_LerpTarget :type "Float (double-precision)"))
  ;[1 1 1] Start Camera Timer Event
  (set `self.CameraLerpStart` (`self.DesiredCameraPosition`))
  (set `self.CameraLerpTarget` CameraLerpTarget)
  (set `self.FOVLerpStart` (`self.TargetCameraFOV`))
  (set `self.FOVLerpTarget` FOV_LerpTarget)
  (set `self.CameraPositionTime` 0.0)
  (set `self.TP_To_FP_Alpha` 0.0)
  (bind _returnvalue (`KismetSystemLibrary.K2_SetTimerDelegate` (`|CreateDelegate` :!event `Camera_Position_Timer`) 0.016667 true))
  (set `self.CameraPositionTimerHandle` _returnvalue))

(event `Camera_Position_Timer`
  (bind _returnvalue (`CurveFloat.GetFloatValue` (`self.CameraPositionCurve`) (`self.CameraPositionTime`)))
  ;[1 1 1] Start Camera Timer Event
  (set `self.CameraPositionTime` (`KismetMathLibrary.FClamp` (+ (`self.CameraPositionTime`) 0.016667) 0.0 (`.MaxTime` (`CurveBase.GetTimeRange` (`self.CameraPositionCurve`)))))
  (set `self.DesiredCameraPosition` (`KismetMathLibrary.VLerp` (`self.CameraLerpStart`) (`self.CameraLerpTarget`) (`CurveFloat.GetFloatValue` (`self.CameraPositionCurve`) (`self.CameraPositionTime`))))
  (set `self.TargetCameraFOV` (`KismetMathLibrary.Lerp` (`self.FOVLerpStart`) (`self.FOVLerpTarget`) _returnvalue))
  (if (`self.IsFirstPerson?`)
    (set `self.TP_To_FP_Alpha` (`KismetMathLibrary.FClamp` _returnvalue))
    (if (`KismetMathLibrary.NearlyEqual_FloatFloat` _returnvalue 1.0 0.001)
      (message `/Game/UltimateShooterKit/Blueprints/Data/Interfaces/BP_PlayerPawnInterface.On_Perspective_Changed` (`self.GetOwningPawn`) true))
    (elif (not (`self.IsADS?`))
      (message `/Game/UltimateShooterKit/Blueprints/Data/Interfaces/BP_PlayerPawnInterface.On_Perspective_Changed` (`self.GetOwningPawn`) false)))
  (if (== (`.MaxTime` (`CurveBase.GetTimeRange` (`self.CameraPositionCurve`))) (`self.CameraPositionTime`))
    (`KismetSystemLibrary.K2_ClearAndInvalidateTimerHandle` (`self.CameraPositionTimerHandle`))))

(event `self.Update_Perspective`
  (params (IsFirstPerson :type Boolean))
  (bind ((`TPPCameraPosition_25_BC220C244C070F1D70C33A8CF2BBD23C` _tppcameraposition) (`TPPAimCameraPosition_28_7910E5814ED69593F5F18D98B478F38D` _tppaimcameraposition) (`TPPFOV_19_240B347A4EA971B806A7AB91D0A4BFC2` _tppfov) (`TPPAimFOV_31_0AC1E3BE4CBF932D997A9D82A9E3C815` _tppaimfov) (`FPPFOV_21_D3A933C340CDC2D41FD20AA72C238C14` _fppfov)) (break `/Game/UltimateShooterKit/Blueprints/Data/Structures/CameraStructs/Struct_CameraSettings` (select `bool` (`self.ShoulderSwitchedTemporary`) :`false` (`self.MakeCameraSettings`) :`true` (`self.MakeCustomCameraSettings` (`self.ShoulderOnLeft`)))))
  ;[1 1 1] Update Perspective
  (set `self.IsFirstPerson?` IsFirstPerson)
  (if (not (`self.IsADS?`))
    (`self.Start_Camera_Timer` (`KismetMathLibrary.SelectVector` (0.0 0.0 0.0) (`KismetMathLibrary.SelectVector` _tppaimcameraposition _tppcameraposition (`self.IsAiming?`)) (`self.IsFirstPerson?`)) (`KismetMathLibrary.SelectFloat` _fppfov (`KismetMathLibrary.SelectFloat` _tppaimfov _tppfov (`self.IsAiming?`)) (`self.IsFirstPerson?`)))))

(event `self.On_Aim`
  (params (`IsAim?` :type Boolean))
  (bind _isaiming_ (`self.IsAiming?`))
  (bind ((`TPPCameraPosition_25_BC220C244C070F1D70C33A8CF2BBD23C` _tppcameraposition) (`TPPAimCameraPosition_28_7910E5814ED69593F5F18D98B478F38D` _tppaimcameraposition) (`TPPFOV_19_240B347A4EA971B806A7AB91D0A4BFC2` _tppfov) (`TPPAimFOV_31_0AC1E3BE4CBF932D997A9D82A9E3C815` _tppaimfov)) (break `/Game/UltimateShooterKit/Blueprints/Data/Structures/CameraStructs/Struct_CameraSettings` (select `bool` (`self.ShoulderSwitchedTemporary`) :`false` (`self.MakeCameraSettings`) :`true` (`self.MakeCustomCameraSettings` (`self.ShoulderOnLeft`)))))
  ;[1 1 1] Handle Aim State
  (set `self.IsAiming?` `IsAim?`)
  (if (and (not (`self.IsFirstPerson?`)) (not (`self.IsADS?`)))
    (`self.Start_Camera_Timer` (`KismetMathLibrary.SelectVector` _tppaimcameraposition _tppcameraposition _isaiming_) (`KismetMathLibrary.SelectFloat` _tppaimfov _tppfov _isaiming_))))

(event `self.Update_Shoulder`
  (bind _camerasettings (`self.CameraSettings`))
  (bind _isaiming_ (`self.IsAiming?`))
  (bind ((`TPPCameraPosition_25_BC220C244C070F1D70C33A8CF2BBD23C` _tppcameraposition) (`TPPAimCameraPosition_28_7910E5814ED69593F5F18D98B478F38D` _tppaimcameraposition) (`TPPFOV_19_240B347A4EA971B806A7AB91D0A4BFC2` _tppfov) (`TPPAimFOV_31_0AC1E3BE4CBF932D997A9D82A9E3C815` _tppaimfov)) (break `/Game/UltimateShooterKit/Blueprints/Data/Structures/CameraStructs/Struct_CameraSettings` (`self.MakeCameraSettings`)))
  ;[1 1 1] Switch Shoulder Events
  (setmembers `/Game/UltimateShooterKit/Blueprints/Data/Structures/CameraStructs/Struct_CameraSettings` :`StructRef` _camerasettings :`Use Left Shoulder` (not (`.UseLeftShoulder_1_DD21E3CA4E574A9172EE2293BA63EE1A` (break `/Game/UltimateShooterKit/Blueprints/Data/Structures/CameraStructs/Struct_CameraSettings` _camerasettings))))
  (if (and (not (`self.IsFirstPerson?`)) (not (`self.IsADS?`)))
    (`self.Start_Camera_Timer` (`KismetMathLibrary.SelectVector` _tppaimcameraposition _tppcameraposition _isaiming_) (`KismetMathLibrary.SelectFloat` _tppaimfov _tppfov _isaiming_))))

(event `self.Update_Shoulder_Temporary`
  (params (ToLeft :type Boolean) (Reset :type Boolean))
  (bind _isaiming_ (`self.IsAiming?`))
  (bind _isaiming__2 (`self.IsAiming?`))
  (bind ((`TPPCameraPosition_25_BC220C244C070F1D70C33A8CF2BBD23C` _tppcameraposition) (`TPPAimCameraPosition_28_7910E5814ED69593F5F18D98B478F38D` _tppaimcameraposition) (`TPPFOV_19_240B347A4EA971B806A7AB91D0A4BFC2` _tppfov) (`TPPAimFOV_31_0AC1E3BE4CBF932D997A9D82A9E3C815` _tppaimfov)) (break `/Game/UltimateShooterKit/Blueprints/Data/Structures/CameraStructs/Struct_CameraSettings` (`self.MakeCameraSettings`)))
  (bind ((`TPPCameraPosition_25_BC220C244C070F1D70C33A8CF2BBD23C` _tppcameraposition_2) (`TPPAimCameraPosition_28_7910E5814ED69593F5F18D98B478F38D` _tppaimcameraposition_2) (`TPPFOV_19_240B347A4EA971B806A7AB91D0A4BFC2` _tppfov_2) (`TPPAimFOV_31_0AC1E3BE4CBF932D997A9D82A9E3C815` _tppaimfov_2)) (break `/Game/UltimateShooterKit/Blueprints/Data/Structures/CameraStructs/Struct_CameraSettings` (`self.CameraSettings`)))
  ;[1 1 1] Switch Shoulder Events
  (if Reset
    (set `self.ShoulderSwitchedTemporary` false)
    (if (and (not (`self.IsFirstPerson?`)) (not (`self.IsADS?`)))
      (`self.Start_Camera_Timer` (`KismetMathLibrary.SelectVector` _tppaimcameraposition _tppcameraposition _isaiming_) (`KismetMathLibrary.SelectFloat` _tppaimfov _tppfov _isaiming_)))
    (elif (!= ToLeft (`.UseLeftShoulder_1_DD21E3CA4E574A9172EE2293BA63EE1A` (break `/Game/UltimateShooterKit/Blueprints/Data/Structures/CameraStructs/Struct_CameraSettings` (`self.MakeCameraSettings`))))
      (set `self.ShoulderOnLeft` ToLeft)
      (set `self.ShoulderSwitchedTemporary` true)
      (if (and (not (`self.IsFirstPerson?`)) (not (`self.IsADS?`)))
        (`self.Start_Camera_Timer` (`KismetMathLibrary.SelectVector` (`self.FindShoulder` ToLeft _tppaimcameraposition_2) (`self.FindShoulder` ToLeft _tppcameraposition_2) _isaiming__2) (`KismetMathLibrary.SelectFloat` _tppaimfov_2 _tppfov_2 _isaiming__2))))))

(fn `ApplyPivotOffset`
  (params (ToVec :type "Vector Structure") (InRot :type "Rotator Structure"))
  (returns (ReturnValue :type "Vector Structure"))
  (bind (_defaultpivotoffset_x _defaultpivotoffset_y _defaultpivotoffset_z) (`KismetMathLibrary.BreakVector` (`self.DefaultPivotOffset`)))
  ;[1 1 1] Add Offset To The Pivot
  (return (+ ToVec (* (`KismetMathLibrary.GetForwardVector` InRot) _defaultpivotoffset_x) (* (`KismetMathLibrary.GetRightVector` InRot) _defaultpivotoffset_y) (* (`KismetMathLibrary.GetUpVector` InRot) _defaultpivotoffset_z))))

(fn `BlueprintUpdateCamera`
  (params (CameraTarget :type "Actor Object Reference"))
  (returns (NewCameraLocation :type "Vector Structure") (NewCameraRotation :type "Rotator Structure") (NewCameraFOV :type "Float (double-precision)") (ReturnValue :type Boolean))
  (bind _targetcamerarotation (`self.TargetCameraRotation`))
  (bind (_returnvalue_x _returnvalue_y _returnvalue_z) (`KismetMathLibrary.BreakVector` (+ (`self.DefaultCameraOffset`) (`self.DesiredCameraPosition`))))
  (bind (_limitonz _defaultinterpolationtime _aiminterpolationtime) (break `/Game/UltimateShooterKit/Blueprints/Data/Structures/CameraStructs/Struct_CameraChickenHead` (`.ChickenHeadSetup_15_C2C7BB4D49A74E1C3F190FBA657B6486` (break `/Game/UltimateShooterKit/Blueprints/Data/Structures/CameraStructs/Struct_CameraSettings` (`self.MakeCameraSettings`)))))
  (if (`self.ActorHasTag` CameraTarget "ShooterCharacter")
    (bind _returnvalue (message `/Game/UltimateShooterKit/Blueprints/Data/Interfaces/BP_PlayerPawnInterface.GetPawnMesh` (`local.CameraTarget`)))
    (`/Engine/EditorBlueprintResources/StandardMacros.IsValid` _returnvalue
      (:`Is Valid`
        (bind (_returnvalue_location _returnvalue_rotation) (`KismetMathLibrary.BreakTransform` (`SceneComponent.GetSocketTransform` _returnvalue "Camera" "RTS_World")))
        (set `self.PivotLocation` (`self.MakeInterpolatedCameraSocket` (`self.ApplyPivotOffset` _returnvalue_location _returnvalue_rotation) _limitonz (`KismetMathLibrary.SelectFloat` _aiminterpolationtime _defaultinterpolationtime (or (`self.IsAiming?`) (`self.IsADS?`)))))
        (`|ExecutionSequence`
          (:`then_0`
            (set `self.TargetCameraRotation` (`Controller.GetControlRotation` (`self.GetOwningPlayerController`))))
          (:`then_1`
            (set `self.TargetCameraLocation` (+ (`self.PivotLocation`) (* (`KismetMathLibrary.GetForwardVector` _targetcamerarotation) _returnvalue_x) (* (`KismetMathLibrary.GetRightVector` _targetcamerarotation) _returnvalue_y) (* (`KismetMathLibrary.GetUpVector` _targetcamerarotation) _returnvalue_z))))
          (:`then_2`
            (bind _outhit (`KismetSystemLibrary.SphereTraceSingle` (`self.PivotLocation`) (`self.TargetCameraLocation`) 10.0 "TraceTypeQuery2"))
            (bind (_bblockinghit _binitialoverlap _time _distance _location _impactpoint _normal _impactnormal _physmat _hitactor _hitcomponent _hitbonename _hititem _faceindex _tracestart _traceend) (`GameplayStatics.BreakHitResult` _outhit))
            (if (and _bblockinghit (not _binitialoverlap))
              (set `self.TargetCameraLocation` (+ (- _location _traceend) (`self.TargetCameraLocation`)))))
          (:`then_3`
            (return (`self.TargetCameraLocation`) (`self.TargetCameraRotation`) (`self.TargetCameraFOV`) true))))
      (:`Is Not Valid`
        ;[1 1 1] Run Parent Function to return the default camera parameters
        (bind (_newcameralocation _newcamerarotation _newcamerafov _returnvalue_2) (`parent.BlueprintUpdateCamera` (`local.CameraTarget`) :!label _label))
        (return _newcameralocation _newcamerarotation _newcamerafov _returnvalue_2)))
    (else
      (goto _label))))

(fn `FindShoulder`
  (params (IsLeftShoulder :type Boolean) (InVec :type "Vector Structure"))
  (returns (ReturnValue :type "Vector Structure"))
  (bind _returnvalue (`KismetMathLibrary.Abs` (.y InVec)))
  ;[1 1 1] This Will Convert The Values According To The Selected Shoulder
  (return (`KismetMathLibrary.MakeVector` (* (`KismetMathLibrary.Abs` (.x InVec)) -1.0) (`KismetMathLibrary.SelectFloat` (* _returnvalue -1.0) _returnvalue (`local.IsLeftShoulder`)) (.z InVec))))

(fn `Get_PostProcessComponent`
  (returns (ReturnValue :type "PostProcessComponent Object Reference"))
  (return (`self.PostProcess`)))

(fn `GetOverlayAnimInstance`
  (params (InTag :type Name :default "ShooterOverlay"))
  (returns (ReturnValue :type "AnimInstance Object Reference"))
  (bind _returnvalue (`self.GetOwningPawn`))
  (`/Engine/EditorBlueprintResources/StandardMacros.IsValid` _returnvalue
    (:`Is Valid`
      (bind _returnvalue_2 (message `/Game/UltimateShooterKit/Blueprints/Data/Interfaces/BP_PlayerPawnInterface.GetPawnMesh` _returnvalue))
      (return (`AnimInstance.GetLinkedAnimGraphInstanceByTag` (`SkeletalMeshComponent.GetAnimInstance` _returnvalue_2) InTag)))))

(fn `GetOwningPawn`
  (returns (ReturnValue :type "Pawn Object Reference"))
  (bind _returnvalue (`self.GetOwningPlayerController`))
  (`/Engine/EditorBlueprintResources/StandardMacros.IsValid` _returnvalue
    (:`Is Valid`
      (return (`Controller.K2_GetPawn` _returnvalue)))))

(fn `MakeCameraSettings`
  (returns (ReturnValue :type "/Game/UltimateShooterKit/Blueprints/Data/Structures/CameraStructs/Struct_CameraSettings Structure"))
  (bind ((`UseLeftShoulder_1_DD21E3CA4E574A9172EE2293BA63EE1A` _useleftshoulder) (`TPPCameraPosition_25_BC220C244C070F1D70C33A8CF2BBD23C` _tppcameraposition) (`TPPAimCameraPosition_28_7910E5814ED69593F5F18D98B478F38D` _tppaimcameraposition)) (break `/Game/UltimateShooterKit/Blueprints/Data/Structures/CameraStructs/Struct_CameraSettings` (`self.CameraSettings`)))
  ;[1 1 1] Make Sure It's Using Correct Values For Each Shoulder
  (bind _structout (setmembers `/Game/UltimateShooterKit/Blueprints/Data/Structures/CameraStructs/Struct_CameraSettings` :`StructRef` (`self.CameraSettings`) :`TPP Camera Position` (`self.FindShoulder` _useleftshoulder _tppcameraposition) :`TPP Aim Camera Position` (`self.FindShoulder` _useleftshoulder _tppaimcameraposition)))
  (return _structout))

(fn `MakeCustomCameraSettings`
  (params (IsLeftShoulder :type Boolean))
  (returns (ReturnValue :type "/Game/UltimateShooterKit/Blueprints/Data/Structures/CameraStructs/Struct_CameraSettings Structure"))
  (bind ((`TPPCameraPosition_25_BC220C244C070F1D70C33A8CF2BBD23C` _tppcameraposition) (`TPPAimCameraPosition_28_7910E5814ED69593F5F18D98B478F38D` _tppaimcameraposition)) (break `/Game/UltimateShooterKit/Blueprints/Data/Structures/CameraStructs/Struct_CameraSettings` (`self.CameraSettings`)))
  ;[1 1 1] Convert Values According To The Desired Shoulder
  (bind _structout (setmembers `/Game/UltimateShooterKit/Blueprints/Data/Structures/CameraStructs/Struct_CameraSettings` :`StructRef` (`self.CameraSettings`) :`TPP Camera Position` (`self.FindShoulder` IsLeftShoulder _tppcameraposition) :`TPP Aim Camera Position` (`self.FindShoulder` IsLeftShoulder _tppaimcameraposition)))
  (return _structout))

(fn `MakeInterpolatedCameraSocket`
  (params (InVec :type "Vector Structure") (Threshold :type "Float (double-precision)" :default 20.0) (InterpSpeed :type "Float (double-precision)" :default 2.0))
  (returns (ReturnValue :type "Vector Structure"))
  (bind _threshold (`local.Threshold`))
  (bind _z (.z (`local.InVec`)))
  (bind _returnvalue (`KismetMathLibrary.VInterpTo` (`self.PivotLocation`) (`local.InVec`) 0.016667 (`local.InterpSpeed`)))
  ;[1 1 1] It Will Help To Keep Camera Steady On Instant Z Axis Changes
  (return (`KismetMathLibrary.MakeVector` (.x (`local.InVec`)) (.y (`local.InVec`)) (`KismetMathLibrary.FClamp` (.z (`KismetMathLibrary.SelectVector` (`local.InVec`) (`KismetMathLibrary.SelectVector` (`KismetMathLibrary.VLerp` _returnvalue (`local.InVec`) (`self.TP_To_FP_Alpha`)) _returnvalue (`self.IsFirstPerson?`)) (`self.IsADS?`))) (- _z _threshold) (+ _z _threshold)))))

(fn `UserConstructionScript`)