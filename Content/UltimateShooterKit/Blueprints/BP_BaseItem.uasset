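; Base item actor for weapons, attachments and consumables, registering with the local character's inventory as an interactable on overlap.
; Builds its mesh and default weapon attachments from a data table row, preferring replicated MasterItemInfo to survive network relevancy.
; Tracks weapon clip and fire mode, and swaps attachments by type.
; Highlighting adds an interaction widget and custom-depth outline in rarity or custom color, while drops use temporary projectile movement.
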(event `self.UpdateMasterItemInfo`
  (params (NewItemInfo :type "/Game/UltimateShooterKit/Blueprints/Data/Structures/Struct_MasterItem Structure"))
  ;[1 1 1] Update Master Item Info - Relevancy Update
  (set `self.MasterItemInfo` NewItemInfo))

(event `self.ReceiveBeginPlay`
  ;[1 1 1] Reconstruct Item On Begin Play
  (`self.UpdateCurrentState`))

(event `self.AddProjectileMovement`
  (bind (_returnvalue_roll _returnvalue_pitch _returnvalue_yaw) (`KismetMathLibrary.BreakRotator` (`self.K2_GetActorRotation`)))
  ;[1 1 1] Add Projectile Movement Component
  (`self.K2_SetActorRotation` (`KismetMathLibrary.MakeRotator` 0.0 0.0 (+ _returnvalue_yaw (`KismetMathLibrary.RandomFloatInRange` -25.0 25.0))))
  (set `PrimitiveComponent.bGenerateOverlapEvents` false (`self.OverlapCollision`))
  (`PrimitiveComponent.IgnoreActorWhenMoving` (`self.RootCollision`) self true)
  (`self.SetReplicateMovement` true)
  (bind _returnvalue (`AddComponent|NODE_AddProjectileMovementComponent-0`))
  (bind _output_get (set `self.ProjectileMovementComp` _returnvalue))
  (add `ProjectileMovementComponent.OnProjectileStop` _output_get (delegate `On_Bounce_Stop`)))

(event `On_Bounce_Stop`
  (params (ImpactResult :type "HitResult Structure (by ref)"))
  ;[1 1 1] Add Projectile Movement Component
  (`ActorComponent.K2_DestroyComponent` (`self.ProjectileMovementComp`))
  (`self.SetReplicateMovement` false)
  (set `PrimitiveComponent.bGenerateOverlapEvents` true (`self.OverlapCollision`)))

(event `Update_Highlight_Color`
  (params (Value :type "LinearColor Structure"))
  ;[1 1 1] Update Post Process Color
  (`/Engine/EditorBlueprintResources/StandardMacros.IsValid` (`self.PostProcessMaterialInstance`)
    (:`Is Valid`
      _)
    (:`Is Not Valid`
      (bind _returnvalue (`KismetMaterialLibrary.CreateDynamicMaterialInstance` "/Game/UltimateShooterKit/Environment/Materials/SceneDepth/M_OutlineMaterial.M_OutlineMaterial"))
      (set `self.PostProcessMaterialInstance` _returnvalue)))
  (`MaterialInstanceDynamic.SetVectorParameterValue` (`self.PostProcessMaterialInstance`) "Outline Color" Value)
  (bind _returnvalue_2 (message `/Game/UltimateShooterKit/Blueprints/Data/Interfaces/BP_CameraManagerInterface.Get_PostProcessComponent` (`GameplayStatics.GetPlayerCameraManager` 0)))
  (bind _structout (setmembers `PostProcessSettings` :`StructRef` (`PostProcessComponent.Settings` _returnvalue_2) :`WeightedBlendables` (make `WeightedBlendables` (`|MakeArray` (make `WeightedBlendable` 1.0 (`self.PostProcessMaterialInstance`))))))
  (set `PostProcessComponent.Settings` _structout _returnvalue_2))

(event `SR_Update_Current_Clip`
  (params (Increase :type Boolean) (Amount :type Integer))
  (bind _currentclip (`self.CurrentClip`))
  ;[1 1 1] Update Clip Events
  (bind _asmasterweapon (`/Game/UltimateShooterKit/Blueprints/Data/Libraries/BP_ShooterFL.GetItemAsWeapon` (`self.ConstructInfo`)))
  (set `self.CurrentClip` (`KismetMathLibrary.Clamp` (`KismetMathLibrary.SelectInt` (+ _currentclip Amount) (- _currentclip Amount) Increase) 0 (`.MaxClip_6_779A517E45536CC863616F84442ED976` (break `/Game/UltimateShooterKit/Blueprints/Data/Structures/WeaponStructures/Struct_ClipSettings` (`.ClipSettings_5_A0EE4DEE4958C4EB5787FC8DB23EE5BD` (break `/Game/UltimateShooterKit/Blueprints/Data/Structures/Struct_MasterWeapon` _asmasterweapon)))))))

(event `self.Update_FireMode`
  ;[1 1 1] Update Fire Mode
  (bind _asmasterweapon (`/Game/UltimateShooterKit/Blueprints/Data/Libraries/BP_ShooterFL.GetItemAsWeapon` (`self.ConstructInfo`)))
  (bind ((`CanSingleFire_20_25CBE5CA45A5DB93C9F99CBEA65BD2E5` _cansinglefire) (`CanBurstFire_22_19552468497992B39FCDB187B09EAF09` _canburstfire) (`CanAutoFire_24_A8EE1A2D4DBA2DE04C001783793503D2` _canautofire)) (break `/Game/UltimateShooterKit/Blueprints/Data/Structures/WeaponStructures/Struct_ShootingSettings` (`.ShootingSettings_8_CB8B4B0545798B5DD72DCD835AA243D4` (break `/Game/UltimateShooterKit/Blueprints/Data/Structures/Struct_MasterWeapon` _asmasterweapon))))
  (set `self.CurrentFireMode` (select `/Game/UltimateShooterKit/Blueprints/Data/Enumerations/Enum_FireModes` (`self.CurrentFireMode`) :`NewEnumerator0` (select `bool` _cansinglefire :`false` (select `bool` _canburstfire :`false` (select `bool` _canautofire :`false` "NewEnumerator0" :`true` "NewEnumerator3" :!type "/Game/UltimateShooterKit/Blueprints/Data/Enumerations/Enum_FireModes Enum") :`true` "NewEnumerator2") :`true` "NewEnumerator1") :`NewEnumerator1` (select `bool` _canburstfire :`false` (select `bool` _canautofire :`false` "NewEnumerator1" :`true` "NewEnumerator3" :!type "/Game/UltimateShooterKit/Blueprints/Data/Enumerations/Enum_FireModes Enum") :`true` "NewEnumerator2") :`NewEnumerator2` (select `bool` _canautofire :`false` (select `bool` _cansinglefire :`false` "NewEnumerator2" :`true` "NewEnumerator1" :!type "/Game/UltimateShooterKit/Blueprints/Data/Enumerations/Enum_FireModes Enum") :`true` "NewEnumerator3") :`NewEnumerator3` (select `bool` _cansinglefire :`false` (select `bool` _canburstfire :`false` "NewEnumerator3" :`true` "NewEnumerator2" :!type "/Game/UltimateShooterKit/Blueprints/Data/Enumerations/Enum_FireModes Enum") :`true` "NewEnumerator1"))))

(event `self.Update_CurrentClip`
  (params (Increase :type Boolean) (Amount :type Integer))
  ;[1 1 1] Update Clip Events
  (`self.SR_Update_Current_Clip` Increase Amount))

(event `self.OverlapCollision.OnComponentBeginOverlap`
  (params (OverlappedComponent :type "PrimitiveComponent Object Reference") (OtherActor :type "Actor Object Reference") (OtherComp :type "PrimitiveComponent Object Reference") (OtherBodyIndex :type Integer) (bFromSweep :type Boolean) (SweepResult :type "HitResult Structure (by ref)"))
  ;[1 1 1] Overlap Events - Adds/Removes Interactables For Inventory Component
  (bind _ascharacter (cast `Character` OtherActor))
  (if (`Pawn.IsLocallyControlled` _ascharacter)
    (`/Game/UltimateShooterKit/Blueprints/Components/Component_Inventory.SR_Assign_Interactable` (`self.GetComponentByClass` (`Pawn.GetController` _ascharacter) "/Game/UltimateShooterKit/Blueprints/Components/Component_Inventory.Component_Inventory_C") true self)))

(event `self.OverlapCollision.OnComponentEndOverlap`
  (params (OverlappedComponent :type "PrimitiveComponent Object Reference") (OtherActor :type "Actor Object Reference") (OtherComp :type "PrimitiveComponent Object Reference") (OtherBodyIndex :type Integer))
  ;[1 1 1] Overlap Events - Adds/Removes Interactables For Inventory Component
  (bind _ascharacter (cast `Character` OtherActor))
  (if (`Pawn.IsLocallyControlled` _ascharacter)
    (`/Game/UltimateShooterKit/Blueprints/Components/Component_Inventory.SR_Assign_Interactable` (`self.GetComponentByClass` (`Pawn.GetController` _ascharacter) "/Game/UltimateShooterKit/Blueprints/Components/Component_Inventory.Component_Inventory_C") false self)))

(fn `AddAttachment`
  (params (AttachmentToAdd :type "/Game/UltimateShooterKit/Blueprints/Data/Structures/Struct_MasterAttachment Structure"))
  (locals (LocSocketToAttach :type Name :default "None") (LocStaticMesh :type "StaticMeshComponent Object Reference") (LocSkeletalMesh :type "SkeletalMeshComponent Object Reference") (LocAttachment :type "/Game/UltimateShooterKit/Blueprints/Data/Structures/Struct_MasterAttachment Structure"))
  (bind (_attachtosocket _typetouse _skeletalmesh _staticmesh) (break `/Game/UltimateShooterKit/Blueprints/Data/Structures/Common/Struct_MeshToAttach` (`.AttachmentMesh_14_3A13727A432BF8B30D1E178C52014F97` (break `/Game/UltimateShooterKit/Blueprints/Data/Structures/Struct_MasterAttachment` (`local.AttachmentToAdd`)))))
  (bind _output_get (set `local.LocAttachment` AttachmentToAdd))
  (bind (_returnvalue _array_element) (`self.HaveSameAttachment?` (`.AttachmentType_2_59E350234890614B673B249DA9564B77` (break `/Game/UltimateShooterKit/Blueprints/Data/Structures/Struct_MasterAttachment` _output_get))))
  (if _returnvalue
    (`self.RemoveAttachment` _array_element))
  ;[1 1 1] Create A New Component For The Type Of Mesh And Attach It To The Requested Socket Of The Main Mesh
  (set `local.LocSocketToAttach` _attachtosocket)
  (switch `/Game/UltimateShooterKit/Blueprints/Data/Enumerations/Enum_MeshType` _typetouse
    (:`NewEnumerator1`
      (bind _returnvalue_2 (`AddComponent|NODE_AddSkeletalMeshComponent-1`))
      (bind _output_get_2 (set `local.LocSkeletalMesh` _returnvalue_2))
      (`SkinnedMeshComponent.SetSkinnedAssetAndUpdate` _output_get_2 _skeletalmesh true)
      (switch `/Game/UltimateShooterKit/Blueprints/Data/Enumerations/Enum_MeshType` (`.TypeToUse_8_196B7DE4447F57E2D9E1C78A0862A1EF` (break `/Game/UltimateShooterKit/Blueprints/Data/Structures/Common/Struct_MeshTypes` (`.BaseMesh_14_3CD095D74632475BAB9BAEBB6A0E45EF` (break `/Game/UltimateShooterKit/Blueprints/Data/Structures/Common/Struct_BaseItemInfo` (`.BaseItemInfo_2_CB340A8F4F0BD84A99CA3E9CEAD5780E` (break `/Game/UltimateShooterKit/Blueprints/Data/Structures/Struct_MasterItem` (`self.ConstructInfo`)))))))
        (:`NewEnumerator1`
          (`SceneComponent.K2_AttachToComponent` (`local.LocSkeletalMesh`) (`self.BaseSMComponent`) (`local.LocSocketToAttach`) "SnapToTarget" "SnapToTarget" "KeepRelative" true)
          (bind _structout (setmembers `/Game/UltimateShooterKit/Blueprints/Data/Structures/Struct_MasterAttachment` :`StructRef` (`local.LocAttachment`) :`SceneComponent - NonEdit` (`local.LocSkeletalMesh`)))
          (`KismetArrayLibrary.Array_Add` (`self.CurrentAttachments`) _structout))
        (:`NewEnumerator2`
          (`SceneComponent.K2_AttachToComponent` (`local.LocSkeletalMesh`) (`self.BaseStaticMeshComponent`) (`local.LocSocketToAttach`) "SnapToTarget" "SnapToTarget" "KeepRelative" true)
          (bind _structout_2 (setmembers `/Game/UltimateShooterKit/Blueprints/Data/Structures/Struct_MasterAttachment` :`StructRef` (`local.LocAttachment`) :`SceneComponent - NonEdit` (`local.LocSkeletalMesh`)))
          (`KismetArrayLibrary.Array_Add` (`self.CurrentAttachments`) _structout_2))))
    (:`NewEnumerator2`
      (bind _returnvalue_3 (`AddComponent|NODE_AddStaticMeshComponent-2`))
      (bind _output_get_3 (set `local.LocStaticMesh` _returnvalue_3))
      (`StaticMeshComponent.SetStaticMesh` _output_get_3 _staticmesh)
      (switch `/Game/UltimateShooterKit/Blueprints/Data/Enumerations/Enum_MeshType` (`.TypeToUse_8_196B7DE4447F57E2D9E1C78A0862A1EF` (break `/Game/UltimateShooterKit/Blueprints/Data/Structures/Common/Struct_MeshTypes` (`.BaseMesh_14_3CD095D74632475BAB9BAEBB6A0E45EF` (break `/Game/UltimateShooterKit/Blueprints/Data/Structures/Common/Struct_BaseItemInfo` (`.BaseItemInfo_2_CB340A8F4F0BD84A99CA3E9CEAD5780E` (break `/Game/UltimateShooterKit/Blueprints/Data/Structures/Struct_MasterItem` (`self.ConstructInfo`)))))))
        (:`NewEnumerator1`
          (`SceneComponent.K2_AttachToComponent` (`local.LocStaticMesh`) (`self.BaseSMComponent`) (`local.LocSocketToAttach`) "SnapToTarget" "SnapToTarget" "KeepRelative" true)
          (bind _structout_3 (setmembers `/Game/UltimateShooterKit/Blueprints/Data/Structures/Struct_MasterAttachment` :`StructRef` (`local.LocAttachment`) :`SceneComponent - NonEdit` (`local.LocStaticMesh`)))
          (`KismetArrayLibrary.Array_Add` (`self.CurrentAttachments`) _structout_3))
        (:`NewEnumerator2`
          (`SceneComponent.K2_AttachToComponent` (`local.LocStaticMesh`) (`self.BaseStaticMeshComponent`) (`local.LocSocketToAttach`) "SnapToTarget" "SnapToTarget" "KeepRelative" true)
          (bind _structout_4 (setmembers `/Game/UltimateShooterKit/Blueprints/Data/Structures/Struct_MasterAttachment` :`StructRef` (`local.LocAttachment`) :`SceneComponent - NonEdit` (`local.LocStaticMesh`)))
          (`KismetArrayLibrary.Array_Add` (`self.CurrentAttachments`) _structout_4))))))

(fn `CreateWidgetOnItem`
  (params (WidgetInformation :type "/Game/UltimateShooterKit/Blueprints/Data/Structures/WeaponStructures/Struct_AvailableAttachments Structure"))
  (returns (WidgetReference :type "Widget Object Reference"))
  (locals (LocWidgetComp :type "WidgetComponent Object Reference"))
  (bind ((`CustomizerSocket_5_F01BD2EA4D9A5739EA5C9AB370CC4C8D` _customizersocket) (`CustomizerSocketOffset_8_E1F26A2C4B2921C5A5DB7DA9E26F48A1` _customizersocketoffset)) (break `/Game/UltimateShooterKit/Blueprints/Data/Structures/WeaponStructures/Struct_AvailableAttachments` (`local.WidgetInformation`)))
  (bind _returnvalue (`WidgetComponent.GetUserWidgetObject` (`local.LocWidgetComp`)))
  (bind _returnvalue_2 (`AddComponent|NODE_AddWidgetComponent-0`))
  (bind _output_get (set `local.LocWidgetComp` _returnvalue_2))
  (`SceneComponent.K2_AttachToComponent` _output_get (select `/Game/UltimateShooterKit/Blueprints/Data/Enumerations/Enum_MeshType` (`.TypeToUse_8_196B7DE4447F57E2D9E1C78A0862A1EF` (break `/Game/UltimateShooterKit/Blueprints/Data/Structures/Common/Struct_MeshTypes` (`.BaseMesh_14_3CD095D74632475BAB9BAEBB6A0E45EF` (break `/Game/UltimateShooterKit/Blueprints/Data/Structures/Common/Struct_BaseItemInfo` (`.BaseItemInfo_2_CB340A8F4F0BD84A99CA3E9CEAD5780E` (break `/Game/UltimateShooterKit/Blueprints/Data/Structures/Struct_MasterItem` (`self.ConstructInfo`))))))) :`NewEnumerator1` (`self.BaseSMComponent`) :`NewEnumerator2` (`self.BaseStaticMeshComponent`) :!type "SceneComponent Object Reference") _customizersocket "SnapToTarget" "SnapToTarget" "KeepRelative" true)
  (`SceneComponent.K2_AddLocalOffset` (`local.LocWidgetComp`) _customizersocketoffset false false)
  (`KismetArrayLibrary.Array_Add` (`self.AttachmentWidgets`) (`local.LocWidgetComp`))
  (message `/Game/UltimateShooterKit/Blueprints/Data/Interfaces/BP_WidgetHandlerInterface.UpdateAttachmentCustomizer` _returnvalue (`local.WidgetInformation`))
  (return _returnvalue))

(fn `DestroyAllWidgetsOnItem`
  (returns (Success :type Boolean))
  (for _array_element (`self.AttachmentWidgets`)
    (message `/Game/UltimateShooterKit/Blueprints/Data/Interfaces/BP_WidgetHandlerInterface.RequestDestroy` (`WidgetComponent.GetUserWidgetObject` _array_element) self))
  (return true))

(fn `DestroyHoverWidget`
  (returns (Success :type Boolean))
  (bind _itemwidget (`self.ItemWidget`))
  (`/Engine/EditorBlueprintResources/StandardMacros.IsValid` _itemwidget
    (:`Is Valid`
      (`ActorComponent.K2_DestroyComponent` _itemwidget)
      (return true))))

(fn `Get_CurrentClip`
  (returns (ReturnValue :type Integer))
  (return (`self.CurrentClip`)))

(fn `Get_FireMode`
  (returns (ReturnValue :type "/Game/UltimateShooterKit/Blueprints/Data/Enumerations/Enum_FireModes Enum"))
  (return (`self.CurrentFireMode`)))

(fn `GetCurrentAttachments`
  (returns (ReturnValue :type "Array of /Game/UltimateShooterKit/Blueprints/Data/Structures/Struct_MasterAttachment Structure"))
  (return (`self.CurrentAttachments`)))

(fn `GetItemClassReference`
  (returns (AsBaseItem :type "/Game/UltimateShooterKit/Blueprints/BP_BaseItem Object Reference"))
  (return self))

(fn `GetItemInfo`
  (returns (MainDataTable :type "DataTableRowHandle Structure") (ReturnValue :type "/Game/UltimateShooterKit/Blueprints/Data/Structures/Struct_MasterItem Structure"))
  (return (`self.ItemDataTable`) (`self.ConstructInfo`)))

(fn `GetItemMeshComponents`
  (returns (AsSkeletalMesh :type "SkeletalMeshComponent Object Reference") (AsStaticMesh :type "StaticMeshComponent Object Reference"))
  (return (`self.BaseSMComponent`) (`self.BaseStaticMeshComponent`)))

(fn `HaveSameAttachment?`
  (params (AttachmentType :type "/Game/UltimateShooterKit/Blueprints/Data/Enumerations/Enum_AttachmentTypes Enum" :default "NewEnumerator0"))
  (returns (ReturnValue :type Boolean) (`Array Element` :type "/Game/UltimateShooterKit/Blueprints/Data/Structures/Struct_MasterAttachment Structure"))
  (locals (LocAlreadyHave :type Boolean :default false) (LocArrayElem :type "/Game/UltimateShooterKit/Blueprints/Data/Structures/Struct_MasterAttachment Structure"))
  (for _array_element (`self.CurrentAttachments`)
    (if (`|EnumEquality` (`.AttachmentType_2_59E350234890614B673B249DA9564B77` (break `/Game/UltimateShooterKit/Blueprints/Data/Structures/Struct_MasterAttachment` _array_element)) (`local.AttachmentType`))
      (set `local.LocAlreadyHave` true)
      (set `local.LocArrayElem` _array_element)
      (break)
      (else
        (set `local.LocAlreadyHave` false)
        (set `local.LocArrayElem` (struct)))))
  (return (`local.LocAlreadyHave`) (`local.LocArrayElem`)))

(fn `OnRep_CurrentClip`
  (bind _aspawn (cast `Pawn` (`self.GetOwner`)))
  (`/Game/UltimateShooterKit/Blueprints/Data/Libraries/BP_ShooterML.IsPawnLocallyControlled?` _aspawn
    (:`true`
      (bind _asmasterweapon (`/Game/UltimateShooterKit/Blueprints/Data/Libraries/BP_ShooterFL.GetItemAsWeapon` (`self.ConstructInfo`)))
      (bind _returnvalue (`/Game/UltimateShooterKit/Blueprints/Data/Libraries/BP_ShooterFL.GetInventoryComponent`))
      (bind (_success _returnvalue_2) (`/Game/UltimateShooterKit/Blueprints/Components/Component_Inventory.FindAmmunition` _returnvalue (`.AmmunitionType_8_690F907E41EB37B569527081EB5E14EE` (break `/Game/UltimateShooterKit/Blueprints/Data/Structures/WeaponStructures/Struct_ClipSettings` (`.ClipSettings_5_A0EE4DEE4958C4EB5787FC8DB23EE5BD` (break `/Game/UltimateShooterKit/Blueprints/Data/Structures/Struct_MasterWeapon` _asmasterweapon))))))
      (message `/Game/UltimateShooterKit/Blueprints/Data/Interfaces/BP_HUDInterface.Request_Update_Ammunition_Info` (`PlayerController.GetHUD` (`GameplayStatics.GetPlayerController` 0)) true (`self.CurrentClip`) (`KismetMathLibrary.SelectInt` (`.Amount_2_A9FDD5864C67C8DF191277B04AC98BFF` (break `/Game/UltimateShooterKit/Blueprints/Data/Structures/Struct_InventorySpace` (`.InventorySpace_22_DE34F9104AA47F419158CDA60A7F12DD` (break `/Game/UltimateShooterKit/Blueprints/Data/Structures/Struct_InventoryItems` _returnvalue_2)))) 0 _success)))))

(fn `OnRep_MasterItemInfo`
  (bind _itemwidget (`self.ItemWidget`))
  (set `self.ConstructInfo` (`self.MasterItemInfo`))
  (`/Engine/EditorBlueprintResources/StandardMacros.IsValid` _itemwidget
    (:`Is Valid`
      (bind _aswidget_interactable_item (cast `/Game/UltimateShooterKit/UserInterface/Widget_InteractableItem` (`WidgetComponent.GetUserWidgetObject` _itemwidget)))
      (`/Game/UltimateShooterKit/UserInterface/Widget_InteractableItem.ReConstruct_ItemWidget` _aswidget_interactable_item (`self.MasterItemInfo`)))))

(fn `OnWidgetDestroyed`
  (params (WidgetReference :type "Widget Object Reference"))
  (returns (Success :type Boolean))
  (for _array_element (`self.AttachmentWidgets`)
    (`ActorComponent.K2_DestroyComponent` _array_element))
  (`KismetArrayLibrary.Array_Clear` (`self.AttachmentWidgets`))
  (return true))

(fn `RemoveAttachment`
  (params (AttachmentInfo :type "/Game/UltimateShooterKit/Blueprints/Data/Structures/Struct_MasterAttachment Structure"))
  (`ActorComponent.K2_DestroyComponent` (`.SceneComponent-NonEdit_19_602190654C6F6B671FAD01BF840BB2FB` (break `/Game/UltimateShooterKit/Blueprints/Data/Structures/Struct_MasterAttachment` AttachmentInfo)))
  (`KismetArrayLibrary.Array_RemoveItem` (`self.CurrentAttachments`) AttachmentInfo))

(fn `RemoveExistingMeshes`
  (bind _basestaticmeshcomponent (`self.BaseStaticMeshComponent`))
  (bind _basesmcomponent (`self.BaseSMComponent`))
  (`/Engine/EditorBlueprintResources/StandardMacros.IsValid` _basesmcomponent
    (:`Is Valid`
      (`ActorComponent.K2_DestroyComponent` _basesmcomponent))
    (:`Is Not Valid`
      _))
  (`/Engine/EditorBlueprintResources/StandardMacros.IsValid` _basestaticmeshcomponent
    (:`Is Valid`
      (`ActorComponent.K2_DestroyComponent` _basestaticmeshcomponent))))

(fn `ResetAttachmentToDefault`
  (params (AttachmentType :type "/Game/UltimateShooterKit/Blueprints/Data/Enumerations/Enum_AttachmentTypes Enum" :default "NewEnumerator0"))
  (returns (Success :type Boolean))
  (locals (LocAttachment :type "/Game/UltimateShooterKit/Blueprints/Data/Structures/Struct_MasterAttachment Structure") (LocValid :type Boolean))
  ;[1 1 1] Get All Default Attachments
  (bind _asmasterweapon (`/Game/UltimateShooterKit/Blueprints/Data/Libraries/BP_ShooterFL.GetItemAsWeapon` (`self.ConstructInfo`)))
  (for _array_element (`.DefaultAttachments_25_16CC22D845D4FD7048DCA19F5E8DF173` (break `/Game/UltimateShooterKit/Blueprints/Data/Structures/Struct_MasterWeapon` _asmasterweapon))
    (if (`|EnumEquality` (`.AttachmentType_2_59E350234890614B673B249DA9564B77` (break `/Game/UltimateShooterKit/Blueprints/Data/Structures/Struct_MasterAttachment` _array_element)) (`local.AttachmentType`))
      (set `local.LocAttachment` _array_element)
      (set `local.LocValid` true)
      (break)
      (else
        (set `local.LocValid` false))))
  ;[1 1 1] Reset Attachment To Default One
  (if (`local.LocValid`)
    (`self.AddAttachment` (`local.LocAttachment`))
    (bind _returnvalue (`/Game/UltimateShooterKit/Blueprints/Data/Libraries/BP_ShooterFL.GetInventoryComponent`))
    (`/Game/UltimateShooterKit/Blueprints/Components/Component_Inventory.UpdateHeldWeaponSights` _returnvalue)
    (return true)))

(fn `SelectHighlightColor`
  (returns (ReturnValue :type "LinearColor Structure"))
  (bind (_useraritycolors _itemrarity _customcolor) (break `/Game/UltimateShooterKit/Blueprints/Data/Structures/Struct_ItemRaritySettings` (`.RaritySettings_24_1F3E40E74D4FB13E76B4AF8E00F9BCE9` (break `/Game/UltimateShooterKit/Blueprints/Data/Structures/Common/Struct_BaseItemInfo` (`.BaseItemInfo_2_CB340A8F4F0BD84A99CA3E9CEAD5780E` (break `/Game/UltimateShooterKit/Blueprints/Data/Structures/Struct_MasterItem` (`self.ConstructInfo`)))))))
  (return (select `bool` _useraritycolors :`false` _customcolor :`true` (`BlueprintMapLibrary.Map_Find` (`self.RarityColors`) _itemrarity))))

(fn `UpdateCurrentAttachment`
  (params (AttachmentInfo :type "/Game/UltimateShooterKit/Blueprints/Data/Structures/Struct_MasterAttachment Structure"))
  (returns (Success :type Boolean))
  (`self.AddAttachment` AttachmentInfo)
  (bind _returnvalue (`/Game/UltimateShooterKit/Blueprints/Data/Libraries/BP_ShooterFL.GetInventoryComponent`))
  (`/Game/UltimateShooterKit/Blueprints/Components/Component_Inventory.UpdateHeldWeaponSights` _returnvalue)
  (return true))

(fn `UpdateCurrentState`
  (`self.UpdateItemInfo`)
  (`self.UpdateItemMesh`)
  (`self.UpdateHasOwner` (`self.HasOwner`)))

(fn `UpdateCustomDepth`
  (params (Component :type "SceneComponent Object Reference") (NewValue :type Boolean))
  (`/Engine/EditorBlueprintResources/StandardMacros.IsValid` Component
    (:`Is Valid`
      (bind _asprimitive_component (cast `PrimitiveComponent` Component))
      (`PrimitiveComponent.SetRenderCustomDepth` _asprimitive_component NewValue))))

(fn `UpdateDataTable`
  (params (NewDataTable :type "DataTableRowHandle Structure"))
  (returns (Success :type Boolean))
  (set `self.ItemDataTable` NewDataTable)
  (`self.UpdateItemInfo`)
  (`self.UpdateItemMesh`)
  (return true))

(fn `UpdateHasOwner`
  (params (HasOwner :type Boolean))
  (returns (Success :type Boolean))
  ;[1 1 1] Destroy OverlapBox If It Has Owner
  (set `self.HasOwner` HasOwner)
  (if (`self.HasOwner`)
    (bind _overlapcollision (`self.OverlapCollision`)
      (:`then`
        (`ActorComponent.K2_DestroyComponent` (`self.Billboard`))
        (`ActorComponent.K2_DestroyComponent` _overlapcollision)
        (return true))
      (:`else`))))

(fn `UpdateHighlight`
  (params (Highlighted :type Boolean))
  (returns (Success :type Boolean))
  (bind _itemwidget (`self.ItemWidget`))
  (if (`local.Highlighted`)
    (`/Engine/EditorBlueprintResources/StandardMacros.IsValid` (`self.ItemWidget`)
      (:`Is Not Valid`
        (bind _returnvalue (`AddComponent|NODE_AddWidgetComponent-1`))
        (bind _output_get (set `self.ItemWidget` _returnvalue))
        (bind _aswidget_interactable_item (cast `/Game/UltimateShooterKit/UserInterface/Widget_InteractableItem` (`WidgetComponent.GetUserWidgetObject` _output_get)))
        (`/Game/UltimateShooterKit/UserInterface/Widget_InteractableItem.Display_Interaction_Widget` _aswidget_interactable_item (`self.ConstructInfo`))
        (`self.Update_Highlight_Color` (`self.SelectHighlightColor`))))
    (else
      (`/Engine/EditorBlueprintResources/StandardMacros.IsValid` _itemwidget
        (:`Is Valid`
          (message `/Game/UltimateShooterKit/Blueprints/Data/Interfaces/BP_WidgetHandlerInterface.RequestDestroy` (`WidgetComponent.GetUserWidgetObject` _itemwidget) self)))))
  (`self.UpdateCustomDepth` (`self.BaseSMComponent`) (`local.Highlighted`))
  (`self.UpdateCustomDepth` (`self.BaseStaticMeshComponent`) (`local.Highlighted`))
  (for _array_element (`self.CurrentAttachments`)
    (`self.UpdateCustomDepth` (`.SceneComponent-NonEdit_19_602190654C6F6B671FAD01BF840BB2FB` (break `/Game/UltimateShooterKit/Blueprints/Data/Structures/Struct_MasterAttachment` _array_element)) (`local.Highlighted`)))
  (return true))

(fn `UpdateItemInfo`
  (bind (_datatabletouse_datatable _datatabletouse_rowname) (break `DataTableRowHandle` (break `/Game/UltimateShooterKit/Blueprints/Data/Structures/Struct_MasterItem` (`self.MasterItemInfo`))))
  ;[1 1 1] Find Item Info From Selected Data Table
  (bind _asmasteritem (`/Game/UltimateShooterKit/Blueprints/Data/Libraries/BP_ShooterFL.GetItemInfo` (`self.ItemDataTable`)))
  ;[1 1 1] Update Construction Info ONLY If The RepNotify Variable Is Not Valid - This Will Help To Keep Item Info Updated - Network Relevancy
  (set `self.ConstructInfo` (select `bool` (and (`KismetSystemLibrary.IsValid` _datatabletouse_datatable) (!= _datatabletouse_rowname "None")) :`false` _asmasteritem :`true` (`self.MasterItemInfo`))))

(fn `UpdateItemMesh`
  (bind ((`BaseMesh_14_3CD095D74632475BAB9BAEBB6A0E45EF` _basemesh) (`ItemOffset_21_DCA4AF134F1B7FF6907F9C98DD1AE4EC` _itemoffset)) (break `/Game/UltimateShooterKit/Blueprints/Data/Structures/Common/Struct_BaseItemInfo` (`.BaseItemInfo_2_CB340A8F4F0BD84A99CA3E9CEAD5780E` (break `/Game/UltimateShooterKit/Blueprints/Data/Structures/Struct_MasterItem` (`self.ConstructInfo`)))))
  (bind ((`SkeletalMesh_2_CB340A8F4F0BD84A99CA3E9CEAD5780E` _skeletalmesh) (`StaticMesh_5_80B0EFA84B24B478758D7AB1C2BD29B9` _staticmesh)) (break `/Game/UltimateShooterKit/Blueprints/Data/Structures/Common/Struct_MeshTypes` _basemesh))
  (`self.RemoveExistingMeshes`)
  ;[1 1 1] Skeletal Mesh Selected?
  (set `self.ItemMeshOffset` (.location _itemoffset))
  (set `self.ItemMeshRotation` (.rotation _itemoffset))
  (switch `/Game/UltimateShooterKit/Blueprints/Data/Enumerations/Enum_MeshType` (`.TypeToUse_8_196B7DE4447F57E2D9E1C78A0862A1EF` (break `/Game/UltimateShooterKit/Blueprints/Data/Structures/Common/Struct_MeshTypes` _basemesh))
    (:`NewEnumerator1`
      ;[1 1 1] Add Meshes As Component
      (bind _returnvalue (`AddComponent|NODE_AddSkeletalMeshComponent-0`))
      (bind _output_get (set `self.BaseSMComponent` _returnvalue))
      (`SkinnedMeshComponent.SetSkinnedAssetAndUpdate` _output_get _skeletalmesh true)
      ;[1 1 1] Update Location And Rotation In Local Space
      (`SceneComponent.K2_AddLocalRotation` (`self.BaseSMComponent`) (`self.ItemMeshRotation`) false false)
      (`SceneComponent.K2_AddLocalOffset` (`self.BaseSMComponent`) (`self.ItemMeshOffset`) false false))
    (:`NewEnumerator2`
      (bind _returnvalue_2 (`AddComponent|NODE_AddStaticMeshComponent-0`))
      (bind _output_get_2 (set `self.BaseStaticMeshComponent` _returnvalue_2))
      (`StaticMeshComponent.SetStaticMesh` _output_get_2 _staticmesh)
      (`SceneComponent.K2_AddLocalRotation` (`self.BaseStaticMeshComponent`) (`self.ItemMeshRotation`) false false)
      (`SceneComponent.K2_AddLocalOffset` (`self.BaseStaticMeshComponent`) (`self.ItemMeshOffset`) false false)))
  ;[1 1 1] Add Default Attachments
  (`self.SwitchOnBaseItemType`
    (:`Weapon`
      (bind _asmasterweapon (`/Game/UltimateShooterKit/Blueprints/Data/Libraries/BP_ShooterFL.GetItemAsWeapon` (`self.ConstructInfo`)))
      (for _array_element (`.DefaultAttachments_25_16CC22D845D4FD7048DCA19F5E8DF173` (break `/Game/UltimateShooterKit/Blueprints/Data/Structures/Struct_MasterWeapon` _asmasterweapon))
        (`self.AddAttachment` _array_element)))))

(fn `UpdateVisibility`
  (params (TargetComponent :type "PrimitiveComponent Object Reference") (OnlyOwnerSee :type Boolean) (OwnerNoSee :type Boolean) (CastToShadows :type Boolean))
  (`PrimitiveComponent.SetOwnerNoSee` (`local.TargetComponent`) (`local.OwnerNoSee`))
  (`PrimitiveComponent.SetOnlyOwnerSee` (`local.TargetComponent`) (`local.OnlyOwnerSee`))
  (`PrimitiveComponent.SetCastShadow` (`local.TargetComponent`) (`local.CastToShadows`)))

(fn `UpdateVisibilityOfItem`
  (params (OnlyOwnerSee :type Boolean) (OwnerNoSee :type Boolean) (CastShadow :type Boolean))
  (returns (Success :type Boolean)))

(fn `UserConstructionScript`
  (bind _basesmcomponent (`self.BaseSMComponent`))
  (`self.UpdateItemInfo`)
  (`self.UpdateItemMesh`)
  (`self.UpdateHasOwner` (`self.HasOwner`))
  (`BoxComponent.SetBoxExtent` (`self.RootCollision`) (`.BoxExtent` (`KismetSystemLibrary.GetComponentBounds` (select `bool` (`KismetSystemLibrary.IsValid` _basesmcomponent) :`false` (`self.BaseStaticMeshComponent`) :`true` _basesmcomponent :!type "SceneComponent Object Reference"))) true))