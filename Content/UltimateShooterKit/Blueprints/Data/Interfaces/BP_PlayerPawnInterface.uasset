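; Blueprint interface for the player pawn in the Ultimate Shooter Kit, declaring the calls other objects make on the pawn without implementing them.
; It covers mesh and default data access, item attachment and removal, and shooting, recoil and projectile hit notifications.
; Movement functions set walk, run and sprint speeds, update speed state and supply movement input, alongside lean queries and first-person perspective change notices.
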(fn `AttachNewItem`
  (params (AttachToSocket :type Name) (ItemDataTable :type "DataTableRowHandle Structure"))
  (returns (ReturnValue :type "ChildActorComponent Object Reference"))
  (return null))

(fn `DestroyAttachedItem`
  (params (Reference :type "ChildActorComponent Object Reference"))
  (returns (Success :type Boolean))
  (return false))

(fn `Get_CurrentLeanValues`
  (returns (LeanAmount :type "Float (double-precision)") (WeaponPositionFPP :type "Transform Structure") (WeaponPositionTPP :type "Transform Structure"))
  (return 0.0))

(fn `GetPawnMesh`
  (returns (ReturnValue :type "SkeletalMeshComponent Object Reference"))
  (return null))

(fn `GetPlayerDefaults`
  (returns (ReturnValue :type "/Game/UltimateShooterKit/Blueprints/Data/Structures/PlayerPawn/Struct_MasterPlayerPawn Structure"))
  (return))

(fn `On_Perspective_Changed`
  (params (IsFirstPerson :type Boolean)))

(fn `OnShoot`)

(fn `ReceiveProjectileHitResult`
  (params (HitResult :type "HitResult Structure")))

(fn `RequestMovementInput`
  (returns (ReturnValue :type "Vector2D Structure"))
  (return (0.0 0.0)))

(fn `SetDefaultRunSpeed`
  (params (NewRunSpeed :type "Float (double-precision)")))

(fn `SetDefaultSprintSpeed`
  (params (NewSprintSpeed :type "Float (double-precision)")))

(fn `SetDefaultWalkSpeed`
  (params (NewWalkSpeed :type "Float (double-precision)")))

(fn `UpdateMaxWalkSpeed`
  (params (NewWalkSpeed :type "Float (double-precision)")))

(fn `UpdateRecoilValues`
  (params (Yaw :type "Float (double-precision)") (Pitch :type "Float (double-precision)"))
  (returns (Success :type Boolean))
  (return false))

(fn `UpdateSpeedState`
  (params (NewSpeedState :type "/Game/UltimateShooterKit/Blueprints/Data/Enumerations/Enum_SpeedStates Enum" :default "NewEnumerator0")))