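; Animation notify that plays a surface-dependent footstep sound for a character's left or right foot, shown as "On Footstep".
; When received, it line-traces on Visibility through the chosen foot socket along the mesh's up axis, ignoring the owner.
; The hit's surface type selects a sound from a map, which spawns attached to the mesh with a configurable volume multiplier.
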(fn `GetNotifyName`
  (returns (ReturnValue :type String))
  (return "On Footstep"))

(fn `Received_Notify`
  (params (MeshComp :type "SkeletalMeshComponent Object Reference") (Animation :type "AnimSequenceBase Object Reference"))
  (returns (ReturnValue :type Boolean))
  (bind _returnvalue (* (`KismetMathLibrary.GetUpVector` (`SceneComponent.K2_GetComponentRotation` MeshComp)) 50.0))
  (bind _returnvalue_2 (`SceneComponent.GetSocketLocation` MeshComp (select `bool` (`self.IsLeftFoot`) :`false` "foot_r" :`true` "foot_l" :!type "Name")))
  (bind _outhit (`KismetSystemLibrary.LineTraceSingle` (+ _returnvalue_2 _returnvalue) (- _returnvalue_2 _returnvalue) "TraceTypeQuery1" false (`|MakeArray` (`ActorComponent.GetOwner` MeshComp))))
  (`GameplayStatics.SpawnSoundAttached` (`BlueprintMapLibrary.Map_Find` (`self.SouındsForSurfaces`) (`GameplayStatics.GetSurfaceType` _outhit)) MeshComp "root" (0.0 0.0 0.0) (struct) "SnapToTarget" false (`self.VolumeMultiplier`) 1.0 0.0 "/Game/UltimateShooterKit/Sounds/SoundClassesAndMixes/BP_SoundAttenuation.BP_SoundAttenuation" "/Game/UltimateShooterKit/Sounds/SoundClassesAndMixes/BP_SoundConcurrency.BP_SoundConcurrency")
  (return true))