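; An animation notify, shown as "Equip Handler", that tells a pawn's inventory when an equip animation reaches its handling point.
; When received, it casts the mesh owner to Pawn and continues only for a valid, locally controlled controller.
; It then finds the inventory component on that controller, not the pawn, and passes its Equip variable to OnEquipHandlerTriggered.
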(fn `GetNotifyName`
  (returns (ReturnValue :type String))
  (return "Equip Handler"))

(fn `Received_Notify`
  (params (MeshComp :type "SkeletalMeshComponent Object Reference") (Animation :type "AnimSequenceBase Object Reference"))
  (returns (ReturnValue :type Boolean))
  (bind _aspawn (cast `Pawn` (`ActorComponent.GetOwner` MeshComp)))
  (bind _returnvalue (`Pawn.GetController` _aspawn))
  (`/Engine/EditorBlueprintResources/StandardMacros.IsValid` _returnvalue
    (:`Is Valid`
      (if (`Controller.IsLocalController` _returnvalue)
        (`/Game/UltimateShooterKit/Blueprints/Components/Component_Inventory.On_Equip_Handler_Triggered` (`Actor.GetComponentByClass` _returnvalue "/Game/UltimateShooterKit/Blueprints/Components/Component_Inventory.Component_Inventory_C") (`self.Equip`))
        (return true)))))