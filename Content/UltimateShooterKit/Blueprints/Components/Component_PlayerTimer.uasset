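; Pawn component that acts as a timeline substitute, animating lean with TPP/TFP weapon offsets, mouse recoil, hand recoil and max walk speed.
; Each Start event resets a time value and starts a looping timer at a fixed frame-rate-derived step.
; Timers sample float curves, clearing themselves at curve end.
; Mouse recoil feeds owner pitch/yaw input directly; the others broadcast interpolated values while ticking.
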(event `self.ReceiveBeginPlay`
  (`self.UpdateComponentOwner`))

(event `Start_Update_Lean`
  (params (TargetLeanValue :type "Float (double-precision)") (TPPWeaponOffsetValues :type "/Game/UltimateShooterKit/Blueprints/Data/Structures/PlayerTimerStructures/Struct_MasterTimerValue Structure") (TFPWeaponOffsetValues :type "/Game/UltimateShooterKit/Blueprints/Data/Structures/PlayerTimerStructures/Struct_MasterTimerValue Structure"))
  ;[1 1 1] Update Lean Values
  (set `self.TargetLeanValue` TargetLeanValue)
  (set `self.StartLeanValue` (`self.Current_LeanAmount`))
  (set `self.TPPWeaponOffset_Values` TPPWeaponOffsetValues)
  (set `self.TFPWeaponOffset_Values` TFPWeaponOffsetValues)
  (bind _returnvalue (`self.SetNewTimer` (`|CreateDelegate` :!event `Lean_Timer`) (`self.Lean_CurrentTime`)))
  (set `self.Lean_TimerHandle` _returnvalue))

(event `Lean_Timer`
  (bind (_startvalue _targetvalue) (break `/Game/UltimateShooterKit/Blueprints/Data/Structures/PlayerTimerStructures/Struct_MasterTimerValue` (`self.TPPWeaponOffset_Values`)))
  (bind (_startvalue_2 _targetvalue_2) (break `/Game/UltimateShooterKit/Blueprints/Data/Structures/PlayerTimerStructures/Struct_MasterTimerValue` (`self.TFPWeaponOffset_Values`)))
  ;[1 1 1] Update Lean Values
  (bind _alpha (`self.UpdateCurrentTime` (`self.Lean_Curve`) (`self.Lean_CurrentTime`)))
  (set `self.Current_LeanAmount` (`KismetMathLibrary.Lerp` (`self.StartLeanValue`) (`self.TargetLeanValue`) _alpha))
  (set `self.Current_TPPWeaponOffset` (`KismetMathLibrary.TLerp` _startvalue _targetvalue _alpha))
  (set `self.Current_TFPWeaponOffset` (`KismetMathLibrary.TLerp` _startvalue_2 _targetvalue_2 _alpha))
  (`self.ClearTimer` (`self.Lean_TimerHandle`) (`self.Lean_CurrentTime`) (`self.Lean_Curve`)
    (:`Ticking`
      (`self.OnLeanAmountUpdate` (`self.Current_LeanAmount`) (`self.Current_TFPWeaponOffset`) (`self.Current_TPPWeaponOffset`)))))

(event `Start_Update_Mouse_Recoil`
  (params (Values :type "/Game/UltimateShooterKit/Blueprints/Data/Structures/PlayerTimerStructures/Struct_MasterTimerValue Structure (by ref)"))
  ;[1 1 1] Update Mouse Recoil
  (set `self.MouseRecoil_Values` Values)
  (bind _returnvalue (`self.SetNewTimer` (`|CreateDelegate` :!event `Mouse_Recoil_Timer`) (`self.MouseRecoil_CurrentTime`)))
  (set `self.MouseRecoil_TimerHandle` _returnvalue))

(event `Mouse_Recoil_Timer`
  ;[1 1 1] Update Mouse Recoil
  (bind _alpha (`self.UpdateCurrentTime` (`self.MouseRecoil_Curve`) (`self.MouseRecoil_CurrentTime`)))
  (`Pawn.AddControllerPitchInput` (`self.ComponentOwner`) (* (.x (.scale (`.StartValue_13_88CBFAF84C50C823E3D515ABBF9BB919` (break `/Game/UltimateShooterKit/Blueprints/Data/Structures/PlayerTimerStructures/Struct_MasterTimerValue` (`self.MouseRecoil_Values`))))) -1.0 _alpha))
  (`Pawn.AddControllerYawInput` (`self.ComponentOwner`) (* (.y (.scale (`.StartValue_13_88CBFAF84C50C823E3D515ABBF9BB919` (break `/Game/UltimateShooterKit/Blueprints/Data/Structures/PlayerTimerStructures/Struct_MasterTimerValue` (`self.MouseRecoil_Values`))))) -1.0 _alpha))
  (`self.ClearTimer` (`self.MouseRecoil_TimerHandle`) (`self.MouseRecoil_CurrentTime`) (`self.MouseRecoil_Curve`)))

(event `Start_Update_Hand_Recoil`
  (params (Values :type "/Game/UltimateShooterKit/Blueprints/Data/Structures/PlayerTimerStructures/Struct_MasterTimerValue Structure (by ref)") (HandRecoil_Curve :type "CurveFloat Object Reference"))
  ;[1 1 1] Update Hand Recoil
  (set `self.HandRecoil_Values` Values)
  (bind _output_get (set `self.HandRecoil_Curve` HandRecoil_Curve))
  (`/Engine/EditorBlueprintResources/StandardMacros.IsValid` _output_get
    (:`Is Valid`
      (bind _returnvalue (`self.SetNewTimer` (`|CreateDelegate` :!event `Hand_Recoil_Timer`) (`self.HandRecoil_CurrentTime`)))
      (set `self.HandRecoil_TimerHandle` _returnvalue))))

(event `Hand_Recoil_Timer`
  (bind (_startvalue _targetvalue) (break `/Game/UltimateShooterKit/Blueprints/Data/Structures/PlayerTimerStructures/Struct_MasterTimerValue` (`self.HandRecoil_Values`)))
  ;[1 1 1] Update Hand Recoil
  (bind _alpha (`self.UpdateCurrentTime` (`self.HandRecoil_Curve`) (`self.HandRecoil_CurrentTime`)))
  (`self.ClearTimer` (`self.HandRecoil_TimerHandle`) (`self.HandRecoil_CurrentTime`) (`self.HandRecoil_Curve`)
    (:`Ticking`
      (`self.OnHandRecoilUpdate` (`KismetMathLibrary.TLerp` _startvalue _targetvalue _alpha)))))

(event `Start_Update_Max_Walk_Speed`
  (params (Values :type "/Game/UltimateShooterKit/Blueprints/Data/Structures/PlayerTimerStructures/Struct_MasterTimerValue Structure (by ref)"))
  ;[1 1 1] Update Max Walk Speed
  (set `self.WalkSpeed_Values` Values)
  (bind _returnvalue (`self.SetNewTimer` (`|CreateDelegate` :!event `Max_Walk_Speed_Timer`) (`self.WalkSpeed_CurrentTime`)))
  (set `self.WalkSpeed_TimerHandle` _returnvalue))

(event `Max_Walk_Speed_Timer`
  (bind (_startvalue _targetvalue) (break `/Game/UltimateShooterKit/Blueprints/Data/Structures/PlayerTimerStructures/Struct_MasterTimerValue` (`self.WalkSpeed_Values`)))
  ;[1 1 1] Update Max Walk Speed
  (bind _alpha (`self.UpdateCurrentTime` (`self.WalkSpeed_Curve`) (`self.WalkSpeed_CurrentTime`)))
  (`self.ClearTimer` (`self.WalkSpeed_TimerHandle`) (`self.WalkSpeed_CurrentTime`) (`self.WalkSpeed_Curve`)
    (:`Ticking`
      (`self.OnWalkSpeedUpdate` (.x (.scale (`KismetMathLibrary.TLerp` _startvalue _targetvalue _alpha)))))))

(fn `ConvertFrameRateToDeltaSeconds`
  (returns (ReturnValue :type "Float (double-precision)"))
  (return (/ (`self.MetersPerFrame`) (`self.FrameRate`))))

(fn `SetNewTimer`
  (params (Event :type "Delegate (by ref)") (CurrentTimeReference :type "Float (double-precision) (by ref)"))
  (returns (ReturnValue :type "TimerHandle Structure"))
  (`|VariableSetRef` (`local.CurrentTimeReference`))
  (bind _returnvalue (`KismetSystemLibrary.K2_SetTimerDelegate` (`local.Event`) (`self.ConvertFrameRateToDeltaSeconds`) true))
  (return _returnvalue))

(fn `UpdateComponentOwner`
  (bind _returnvalue (`self.GetOwner`))
  (`/Engine/EditorBlueprintResources/StandardMacros.IsValid` _returnvalue
    (:`Is Valid`
      (bind _aspawn (cast `Pawn` _returnvalue))
      (set `self.ComponentOwner` _aspawn))))

(fn `UpdateCurrentTime`
  (params (Curve :type "CurveFloat Object Reference") (TimeReference :type "Float (double-precision) (by ref)"))
  (returns (Alpha :type "Float (double-precision)"))
  (bind (_mintime _maxtime) (`CurveBase.GetTimeRange` (`local.Curve`)))
  (`|VariableSetRef` (`local.TimeReference`) (`KismetMathLibrary.FClamp` (+ (`local.TimeReference`) (`self.ConvertFrameRateToDeltaSeconds`)) _mintime _maxtime))
  (return (`CurveFloat.GetFloatValue` (`local.Curve`) (`local.TimeReference`))))