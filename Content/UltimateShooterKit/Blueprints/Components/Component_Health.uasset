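; Pawn health component for the shooter kit, tracking health, armor and boost with clamped values.
; It binds to the owner's any-damage event, draining armor first and passing overflow to health.
; Boost drains at a constant rate on a looping 60 Hz timer that converts it into health regeneration.
; RepNotify functions push changes to the local player's HUD, and Apply Damage To Actor also shows a damage direction indicator.
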(event `self.ReceiveBeginPlay`
  ;[1 1 1] Begin Play
  (`self.Set_PawnOwner`)
  (add `Actor.OnTakeAnyDamage` (`self.PossessedPawn`) (`|CreateDelegate` :!event `Bind_Any_Damage`)))

(event `Bind_Any_Damage`
  (params (DamagedActor :type "Actor Object Reference") (Damage :type "Float (double-precision)") (DamageType :type "DamageType Object Reference") (InstigatedBy :type "Controller Object Reference") (DamageCauser :type "Actor Object Reference"))
  ;[1 1 1] Bind OnTakeDamage
  (`self.SR_Apply_Damage` DamagedActor Damage DamageCauser))

(event `SR_Set_Default_Values`
  ;[1 1 1] Update Default Values
  (set `self.CurrentHealth` (`KismetMathLibrary.FClamp` (`self.DefaultHealth`) 0.0 (`self.MaxHealth`)))
  (set `self.CurrentArmor` (`KismetMathLibrary.FClamp` (`self.DefaultArmor`) 0.0 (`self.MaxArmor`)))
  (set `self.CurrentBoost` 0.0)
  (`self.Update_Default_Values_On_Widget`))

(event `Apply_Damage_To_Actor`
  (params (DamagedActor :type "Actor Object Reference") (BaseDamage :type "Float (double-precision)") (DamageCauser :type "Actor Object Reference"))
  ;[1 1 1] Apply Damage To Player Pawn And Create A Damage Indicator
  (`GameplayStatics.ApplyDamage` DamagedActor BaseDamage null DamageCauser)
  (`/Game/UltimateShooterKit/Blueprints/Data/Libraries/BP_ShooterML.IsPawnLocallyControlled?` (`self.PossessedPawn`) true
    (:`true`
      (message `/Game/UltimateShooterKit/Blueprints/Data/Interfaces/BP_HUDInterface.Create_Damage_Indicator` (`PlayerController.GetHUD` (`GameplayStatics.GetPlayerController` 0)) (`Actor.K2_GetActorLocation` DamageCauser)))))

(event `Update_Default_Values_On_Widget`
  ;[1 1 1] Update Default Values
  (message `/Game/UltimateShooterKit/Blueprints/Data/Interfaces/BP_HUDInterface.Request_Update_Health` (`PlayerController.GetHUD` (`GameplayStatics.GetPlayerController` 0)) (`self.CurrentHealth`) (`self.MaxHealth`) false)
  (message `/Game/UltimateShooterKit/Blueprints/Data/Interfaces/BP_HUDInterface.Request_Update_Armor` (`PlayerController.GetHUD` (`GameplayStatics.GetPlayerController` 0)) (`self.CurrentArmor`) (`self.MaxArmor`))
  (message `/Game/UltimateShooterKit/Blueprints/Data/Interfaces/BP_HUDInterface.Request_Update_Boost` (`PlayerController.GetHUD` (`GameplayStatics.GetPlayerController` 0)) 0.0 (`self.MaxBoost`)))

(event `SR_Apply_Damage`
  (params (DamagedActor :type "Actor Object Reference") (BaseDamage :type "Float (double-precision)") (DamageCauser :type "Actor Object Reference"))
  (bind _returnvalue (- (`self.CurrentArmor`) BaseDamage))
  ;[1 1 1] Apply Damage To Player Pawn And Create A Damage Indicator
  (`|ExecutionSequence`
    (:`then_0`
      (if (> (`self.CurrentArmor`) 0.0)
        (if (>= _returnvalue 0.0)
          (set `self.CurrentArmor` (`KismetMathLibrary.FClamp` _returnvalue 0.0 (`self.MaxArmor`)))
          (else
            (set `self.IncreaseHealthWidgetInTime` (not (`KismetSystemLibrary.K2_IsValidTimerHandle` (`self.BoostTimerHandle`))))
            (set `self.CurrentHealth` (`KismetMathLibrary.FClamp` (- (`self.CurrentHealth`) (`KismetMathLibrary.Abs` _returnvalue)) 0.0 (`self.MaxHealth`)))
            (set `self.CurrentArmor` 0.0)))
        (else
          (set `self.CurrentHealth` (`KismetMathLibrary.FClamp` (- (`self.CurrentHealth`) BaseDamage) 0.0 (`self.MaxHealth`)))
          (set `self.IncreaseHealthWidgetInTime` (not (`KismetSystemLibrary.K2_IsValidTimerHandle` (`self.BoostTimerHandle`)))))))))

(event `SR_Add_Health`
  (params (IncreaseAmount :type "Float (double-precision)"))
  ;[1 1 1] Health Event
  (set `self.IncreaseHealthWidgetInTime` (not (`KismetSystemLibrary.K2_IsValidTimerHandle` (`self.BoostTimerHandle`))))
  (set `self.CurrentHealth` (`KismetMathLibrary.FClamp` (+ (`self.CurrentHealth`) IncreaseAmount) 0.0 (`self.MaxHealth`))))

(event `SR_Add_Armor`
  (params (IncreaseAmount :type "Float (double-precision)"))
  ;[1 1 1] Armor Event
  (set `self.CurrentArmor` (`KismetMathLibrary.FClamp` (+ (`self.CurrentArmor`) IncreaseAmount) 0.0 (`self.MaxArmor`))))

(event `SR_Add_Boost`
  (params (IncreaseAmount :type "Float (double-precision)"))
  ;[1 1 1] Boost Event
  (bind _output_get (set `self.CurrentBoost` (`KismetMathLibrary.FClamp` (+ (`self.CurrentBoost`) IncreaseAmount) 0.0 (`self.MaxBoost`))))
  (set `self.BoostToHealthAmount` _output_get)
  (set `self.IncreaseHealthWidgetInTime` false)
  (if (not (`KismetSystemLibrary.K2_IsValidTimerHandle` (`self.BoostTimerHandle`)))
    (bind _returnvalue (`KismetSystemLibrary.K2_SetTimerDelegate` (`|CreateDelegate` :!event `Health_Regeneration_By_Boost_Timer`) 0.016667 true))
    (set `self.BoostTimerHandle` _returnvalue)))

(event `Health_Regeneration_By_Boost_Timer`
  (bind _returnvalue (`KismetMathLibrary.FInterpTo_Constant` (`self.CurrentBoost`) 0.0 0.016667 (/ (`self.BoostToHealthAmount`) (`self.BoostToHealtInSeconds`))))
  ;[1 1 1] Boost Event
  (set `self.CurrentBoost` _returnvalue)
  (set `self.CurrentHealth` (`KismetMathLibrary.FClamp` (+ (`self.CurrentHealth`) (- (`self.CurrentBoost`) _returnvalue)) 0.0 (`self.MaxHealth`)))
  (if (== (`self.CurrentBoost`) 0.0)
    (`KismetSystemLibrary.K2_ClearAndInvalidateTimerHandle` (`self.BoostTimerHandle`))))

(fn `OnRep_CurrentArmor`
  (`/Game/UltimateShooterKit/Blueprints/Data/Libraries/BP_ShooterML.IsPawnLocallyControlled?` (`self.PossessedPawn`) true
    (:`true`
      (message `/Game/UltimateShooterKit/Blueprints/Data/Interfaces/BP_HUDInterface.Request_Update_Armor` (`PlayerController.GetHUD` (`GameplayStatics.GetPlayerController` 0)) (`self.CurrentArmor`) (`self.MaxArmor`)))))

(fn `OnRep_CurrentBoost`
  (`/Game/UltimateShooterKit/Blueprints/Data/Libraries/BP_ShooterML.IsPawnLocallyControlled?` (`self.PossessedPawn`) true
    (:`true`
      (message `/Game/UltimateShooterKit/Blueprints/Data/Interfaces/BP_HUDInterface.Request_Update_Boost` (`PlayerController.GetHUD` (`GameplayStatics.GetPlayerController` 0)) (`self.CurrentBoost`) (`self.MaxBoost`)))))

(fn `OnRep_CurrentHealth`
  (`/Game/UltimateShooterKit/Blueprints/Data/Libraries/BP_ShooterML.IsPawnLocallyControlled?` (`self.PossessedPawn`) true
    (:`true`
      (message `/Game/UltimateShooterKit/Blueprints/Data/Interfaces/BP_HUDInterface.Request_Update_Health` (`PlayerController.GetHUD` (`GameplayStatics.GetPlayerController` 0)) (`self.CurrentHealth`) (`self.MaxHealth`) (`self.IncreaseHealthWidgetInTime`)))))

(fn `Set_PawnOwner`
  (bind _aspawn (cast `Pawn` (`self.GetOwner`)))
  (set `self.PossessedPawn` _aspawn)
  (`self.SR_Set_Default_Values`))