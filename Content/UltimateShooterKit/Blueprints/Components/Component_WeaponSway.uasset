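; Character component that drives procedural first-person weapon sway from aim and movement input, pushed every tick to the "ShooterOverlay" linked anim instance.
; Clamped tilt uses separate hip and aim tuning, while an optional aim-only dead zone accumulates aim delta into offsets.
; Both blend into one interpolated transform, which settles to the dead zone offset or zero without input.
; Interpolation uses a fixed 60 Hz timestep rather than frame delta.
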(event `self.ReceiveTick`
  (params (DeltaSeconds :type "Float (single-precision)"))
  ;[1 1 1] Event Tick | Begin Play
  (`|ExecutionSequence`
    (:`then_0`
      (`self.UpdateFinalSway`))
    (:`then_1`
      (message `/Game/UltimateShooterKit/Blueprints/Data/Interfaces/BP_OverlayAnimBPInterface.Update_WeaponSway` (`self.GetOverlayAnimInstance` "ShooterOverlay") (`self.FinalSwayTransform`)))
    (:`then_2`)))

(event `self.ReceiveBeginPlay`
  ;[1 1 1] Event Tick | Begin Play
  (`|ExecutionSequence`
    (:`then_0`
      (`self.UpdateComponentOwner`))))

(event `Toggle_Dead_Zone`
  (params (Enabled :type Boolean))
  ;[1 1 1] Not In Final State..
  (bind _output_get (set `self.EnableDeadZone` Enabled))
  (if (not _output_get)
    (set `self.DeadZoneRotation` (struct))
    (set `self.DeadZoneLocation` (0.0 0.0 0.0))
    (set `self.CurrentDeadZoneAmount` (0.0 0.0))))

(fn `CalculateDeadZone`
  (bind (_currentdeadzoneamount_x _currentdeadzoneamount_y) (`KismetMathLibrary.BreakVector2D` (`self.CurrentDeadZoneAmount`)))
  (bind (_finalswaytransform_location _finalswaytransform_rotation) (`KismetMathLibrary.BreakTransform` (`self.FinalSwayTransform`)))
  (bind (_deadzoneclamp_left _deadzoneclamp_top _deadzoneclamp_right) (break `Margin` (`self.DeadZoneClamp`)))
  (bind (_deadzoneclamp_left_2 _deadzoneclamp_top_2 _deadzoneclamp_right_2 _deadzoneclamp_bottom) (break `Margin` (`self.DeadZoneClamp`)))
  (bind _deadzonesensitivity (`self.DeadZoneSensitivity`))
  (bind _returnvalue (* (`KismetMathLibrary.FClamp` (+ (.pitch _finalswaytransform_rotation) (* _currentdeadzoneamount_x _deadzonesensitivity)) (* _deadzoneclamp_bottom -1.0) _deadzoneclamp_top_2) -1.0))
  (bind _returnvalue_2 (`KismetMathLibrary.FClamp` (* (+ (.yaw _finalswaytransform_rotation) (* _currentdeadzoneamount_y (* _deadzonesensitivity -1.0))) -1.0) (* _deadzoneclamp_left_2 -1.0) _deadzoneclamp_right_2))
  ;[1 1 1] Reset Dead Zone Values If It's Disabled Or Not Aiming
  (if (and (`self.EnableDeadZone`) (`self.IsAiming?`))
    ;[1 1 1] Calculate Dead Zone
    (set `self.CurrentDeadZoneAmount` (`KismetMathLibrary.ClampAxes2D` (+ (`self.CurrentDeadZoneAmount`) (`self.AimDelta`)) (* (/ _deadzoneclamp_left 2.0) -1.0) (/ _deadzoneclamp_right 2.0)))
    (set `self.DeadZoneRotation` (`KismetMathLibrary.MakeRotator` 0.0 _returnvalue _returnvalue_2))
    (set `self.DeadZoneLocation` (`KismetMathLibrary.MakeVector` 0.0 (/ _returnvalue_2 5.0) (/ _returnvalue 5.0)))
    (else
      (set `self.DeadZoneRotation` (struct))
      (set `self.DeadZoneLocation` (0.0 0.0 0.0))
      (set `self.CurrentDeadZoneAmount` (0.0 0.0)))))

(fn `CalculateTilting`
  (returns (Rotation :type "Rotator Structure") (Location :type "Vector Structure"))
  (locals (LocTiltAroundZ :type "Float (double-precision)") (LocTiltAroundX :type "Float (double-precision)"))
  (bind _movementdelta_x (`KismetMathLibrary.BreakVector2D` (`self.MovementDelta`)))
  (bind _loctiltaroundz (`local.LocTiltAroundZ`))
  (bind (_aimdelta_x _aimdelta_y) (`KismetMathLibrary.BreakVector2D` (`self.AimDelta`)))
  (bind _loctiltaroundx (`local.LocTiltAroundX`))
  (bind (_left _top _right _bottom) (break `Margin` (select `bool` (`self.IsAiming?`) :`false` (`self.TiltClamp`) :`true` (`self.TiltClampOnAim`))))
  (if (`self.EnableTilt`)
    (set `local.LocTiltAroundZ` (`KismetMathLibrary.FClamp` (* (`KismetMathLibrary.SelectFloat` (`self.TiltingSensitivityWithMouseOnAim`) (`self.TiltingSensitivityWithMouse`) (`self.IsAiming?`)) _aimdelta_x -1.0) (* _bottom -1.0) _top))
    (set `local.LocTiltAroundX` (`KismetMathLibrary.FClamp` (+ (* (`KismetMathLibrary.SelectFloat` (`self.TiltingSensitivityWithMouseOnAim`) (`self.TiltingSensitivityWithMouse`) (`self.IsAiming?`)) _aimdelta_y) (* (`KismetMathLibrary.SelectFloat` (`self.TiltingSensitivityWithMovementOnAim`) (`self.TiltingSensitivityWithMovement`) (`self.IsAiming?`)) _movementdelta_x)) (* _left -1.0) _right))
    (return (`KismetMathLibrary.MakeRotator` _loctiltaroundx _loctiltaroundz) (`KismetMathLibrary.MakeVector` 0.0 _loctiltaroundx (* _loctiltaroundz -1.0)))
    (else
      (return (struct) (0.0 0.0 0.0)))))

(fn `GetOverlayAnimInstance`
  (params (InTag :type Name :default "ShooterOverlay"))
  (returns (ReturnValue :type "AnimInstance Object Reference"))
  (bind _returnvalue (message `/Game/UltimateShooterKit/Blueprints/Data/Interfaces/BP_PlayerPawnInterface.GetPawnMesh` (`self.ComponentOwner`)))
  (return (`AnimInstance.GetLinkedAnimGraphInstanceByTag` (`SkeletalMeshComponent.GetAnimInstance` _returnvalue) (`local.InTag`))))

(fn `UpdateAimDelta`
  (params (AimDelta :type "Vector2D Structure"))
  (set `self.AimDelta` AimDelta))

(fn `UpdateAimPose`
  (params (IsAim :type Boolean))
  (set `self.IsAiming?` IsAim))

(fn `UpdateComponentOwner`
  (bind _returnvalue (`self.GetOwner`))
  ;[1 1 1] Update Component Owner Reference
  (`/Engine/EditorBlueprintResources/StandardMacros.IsValid` _returnvalue
    (:`Is Valid`
      (bind _ascharacter (cast `Character` _returnvalue))
      (set `self.ComponentOwner` _ascharacter))))

(fn `UpdateFinalSway`
  (bind (_finalswaytransform_location _finalswaytransform_rotation) (`KismetMathLibrary.BreakTransform` (`self.FinalSwayTransform`)))
  ;[1 1 1] Only Update If Mouse Or Movement Input Is Not Equal To 0
  (if (or (!= (`self.AimDelta`) (0.0 0.0)) (!= (`self.MovementDelta`) (0.0 0.0)))
    ;[1 1 1] Calculate Tilting
    (bind (_rotation _location) (`self.CalculateTilting`))
    ;[1 1 1] Update Final Sway
    (set `self.FinalSwayTransform` (`KismetMathLibrary.MakeTransform` (`KismetMathLibrary.VInterpTo` _finalswaytransform_location (+ _location (`self.DeadZoneLocation`)) 0.016667 (`self.SmoothSway`)) (`KismetMathLibrary.RInterpTo` (`self.DeadZoneRotation`) (`KismetMathLibrary.ComposeRotators` (`KismetMathLibrary.SelectRotator` (struct) _rotation (`self.IsAiming?`)) _finalswaytransform_rotation) 0.016667 (`self.SmoothSway`))))
    ;[1 1 1] Calculate Dead Zone
    (`self.CalculateDeadZone`)
    (else
      ;[1 1 1] Update Only Dead Zone Transform
      (set `self.FinalSwayTransform` (`KismetMathLibrary.TInterpTo` (`self.FinalSwayTransform`) (`KismetMathLibrary.SelectTransform` (`KismetMathLibrary.MakeTransform` (`self.DeadZoneLocation`) (`self.DeadZoneRotation`)) (`KismetMathLibrary.MakeTransform` (0.0 0.0 0.0)) (`self.EnableDeadZone`)) 0.016667 (`self.SmoothSway`))))))

(fn `UpdateMovementDelta`
  (params (MovementDelta :type "Vector2D Structure"))
  (set `self.MovementDelta` MovementDelta))