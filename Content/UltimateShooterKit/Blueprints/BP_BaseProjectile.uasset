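; Base bullet projectile for the shooter kit, with surface-dependent penetration, ricochet, impact effects and flyby sound.
; On bounce, it reports the first hit to its owner, then uses angle and chance to ricochet or penetrate.
; Penetration finds the exit by recursive reverse sphere traces, subtracts kinetic energy by thickness, then rebuilds the movement component there or destroys the bullet.
; AmmunitionInfo supplies visuals and per-surface data; optional debug lines show speed by color.
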(event `self.ReceiveTick`
  (params (DeltaSeconds :type "Float (single-precision)"))
  ;[1 1 1] Event Tick | Begin Play
  (if (`self.EnableDebugLines`)
    (`KismetSystemLibrary.DrawDebugLine` (`self.LastLocation`) (`self.K2_GetActorLocation`) (`self.FindTraceColor` (`MovementComponent.Velocity` (`self.PRMovement`))) (`self.TraceDuration`))
    (set `self.LastLocation` (`self.K2_GetActorLocation`))))

(event `self.ReceiveBeginPlay`
  (bind (_projectilemesh _projectileparticle) (break `/Game/UltimateShooterKit/Blueprints/Data/Structures/WeaponStructures/Struct_AmmoMaster` (`self.AmmunitionInfo`)))
  ;[1 1 1] Event Tick | Begin Play
  (`self.ConstructProjectileMovement` (0.0 0.0 0.0))
  (`PrimitiveComponent.IgnoreActorWhenMoving` (`self.Sphere`) (`self.GetOwner`) true)
  (`StaticMeshComponent.SetStaticMesh` (`self.BulletMesh`) _projectilemesh)
  (`ParticleSystemComponent.SetTemplate` (`self.ParticleSystem`) _projectileparticle)
  (set `self.LastLocation` (`self.K2_GetActorLocation`))
  (`KismetSystemLibrary.Delay` 0.025)
  (set `MovementComponent.Velocity` (`self.BulletDirection`) (`self.PRMovement`))
  (set `ProjectileMovementComponent.InitialSpeed` (`self.BulletInitialSpeed`) (`self.PRMovement`))
  (`KismetSystemLibrary.Delay` 0.0)
  (`SceneComponent.SetHiddenInGame` (`self.BulletMesh`) false false)
  (`SceneComponent.SetHiddenInGame` (`self.ParticleSystem`) false false))

(event `Play_Hit_Effects`
  (params (Bounced :type Boolean) (Hit :type "HitResult Structure (by ref)"))
  (bind (_bblockinghit _binitialoverlap _time _distance _location _impactpoint _normal _impactnormal _physmat _hitactor _hitcomponent _hitbonename) (`GameplayStatics.BreakHitResult` Hit))
  (bind (_lasthittransform_location _lasthittransform_rotation) (`KismetMathLibrary.BreakTransform` (`self.LastHitTransform`)))
  (bind (_lasthittransform_location_2 _lasthittransform_rotation_2) (`KismetMathLibrary.BreakTransform` (`self.LastHitTransform`)))
  (bind (_lasthittransform_location_3 _lasthittransform_rotation_3 _lasthittransform_scale) (`KismetMathLibrary.BreakTransform` (`self.LastHitTransform`)))
  (bind ((`ImpactParticle_21_EDEEF19C49CBDD81E2666DB31CA7B972` _impactparticle) (`RicochetParticle_15_89D96E7747DB386C073C1A976514A131` _ricochetparticle)) (break `/Game/UltimateShooterKit/Blueprints/Data/Structures/WeaponStructures/Struct_AmmoVFX` (`self.FindBulletVFX` (`self.LastHitSurfaceType`))))
  (bind ((`ImpactSound_6_7BDA651A484BD6B28B566DB7F05F5275` _impactsound) (`RicochetSound_8_89D96E7747DB386C073C1A976514A131` _ricochetsound)) (break `/Game/UltimateShooterKit/Blueprints/Data/Structures/WeaponStructures/Struct_AmmoSFX` (`self.FindBulletSFX` (`self.LastHitSurfaceType`))))
  (bind ((`ImpactDecal_12_7BDA651A484BD6B28B566DB7F05F5275` _impactdecal) (`RicochetDecal_18_9DE262E54E701E30CC0052BD356C0CAF` _ricochetdecal)) (break `/Game/UltimateShooterKit/Blueprints/Data/Structures/WeaponStructures/Struct_AmmoVFX` (`self.FindBulletVFX` (`self.LastHitSurfaceType`))))
  (bind _returnvalue (select `bool` (`self.Ricochet?`) :`false` _impactparticle :`true` _ricochetparticle))
  (bind _returnvalue_2 (select `bool` (`self.Ricochet?`) :`false` _impactsound :`true` _ricochetsound))
  (bind (_decalmaterial _decalsizemin_max _lifespan) (break `/Game/UltimateShooterKit/Blueprints/Data/Structures/Common/Struct_DecalSetup` (select `bool` (`self.Ricochet?`) :`false` _impactdecal :`true` _ricochetdecal)))
  (bind (_x _y) (`KismetMathLibrary.BreakVector2D` _decalsizemin_max))
  (bind _returnvalue_3 (`KismetMathLibrary.RandomFloatInRange` _x _y))
  ;[1 1 1] Effects And OnBounce Setup
  (set `self.Ricochet?` Bounced)
  (`self.UpdateHitVars` Hit)
  (`/Engine/EditorBlueprintResources/StandardMacros.IsValid` _returnvalue
    (:`Is Valid`
      (`GameplayStatics.SpawnEmitterAtLocation` _returnvalue _lasthittransform_location_3 (`self.MirroredRotation`) _lasthittransform_scale))
    (:`Is Not Valid`
      _))
  (`/Engine/EditorBlueprintResources/StandardMacros.IsValid` _returnvalue_2
    (:`Is Valid`
      (`GameplayStatics.SpawnSoundAtLocation` _returnvalue_2 _lasthittransform_location_2 _lasthittransform_rotation_2 1.0 1.0 0.0 "/Game/UltimateShooterKit/Sounds/SoundClassesAndMixes/BP_SoundAttenuation.BP_SoundAttenuation" "/Game/UltimateShooterKit/Sounds/SoundClassesAndMixes/BP_SoundConcurrency.BP_SoundConcurrency"))
    (:`Is Not Valid`
      _))
  (`/Engine/EditorBlueprintResources/StandardMacros.IsValid` _decalmaterial
    (:`Is Valid`
      (`GameplayStatics.SpawnDecalAttached` _decalmaterial (`KismetMathLibrary.MakeVector` 3.5 _returnvalue_3 _returnvalue_3) (select `bool` (== (`GameplayStatics.GetObjectClass` _hitactor) "/Script/Engine.Character") :`false` _hitcomponent :`true` (`Character.Mesh` (cast `Character` _hitactor :!pure true)) :!type "SceneComponent Object Reference") _hitbonename (+ _lasthittransform_location (* (`KismetMathLibrary.GetForwardVector` _lasthittransform_rotation) -3.5)) (`KismetMathLibrary.MakeRotator` (`KismetMathLibrary.RandomFloatInRange` 0.0 360.0) (.pitch _lasthittransform_rotation) (.yaw _lasthittransform_rotation)) "KeepWorldPosition" _lifespan))))

(event `On_Custom_PR_Bounced`
  (params (ImpactResult :type "HitResult Structure (by ref)") (ImpactVelocity :type "Vector Structure (by ref)"))
  (bind _lastimpactvelocity (`self.LastImpactVelocity`))
  (bind _prmovement (`self.PRMovement`))
  (bind (_bblockinghit _binitialoverlap _time _distance _location) (`GameplayStatics.BreakHitResult` (`self.LastImpactResult`)))
  ;[1 1 1] Effects And OnBounce Setup
  (set `self.LastImpactResult` ImpactResult)
  (set `self.LastImpactVelocity` ImpactVelocity)
  (`|ExecutionSequence`
    (:`then_0`
      (`/Engine/EditorBlueprintResources/StandardMacros.DoOnce` false
        (:`Completed`
          (message `/Game/UltimateShooterKit/Blueprints/Data/Interfaces/BP_PlayerPawnInterface.ReceiveProjectileHitResult` (`self.GetOwner`) (`self.LastImpactResult`)))))
    (:`then_1`
      _))
  (if (`self.EnableDebugLines`)
    (`KismetSystemLibrary.DrawDebugLine` (`self.LastLocation`) _location (`self.FindTraceColor` (`self.LastImpactVelocity`)) (`self.TraceDuration`))
    (set `self.LastLocation` _location))
  (bind _returnvalue (`self.ShouldPenetrate` (`self.LastImpactResult`) (`self.LastImpactVelocity`)))
  (if _returnvalue
    (`self.Play_Hit_Effects` false (`self.LastImpactResult`))
    (bind (_returnvalue_2 _success _penetrationresult) (`self.CalculateProjectileExitLocation` (`self.LastImpactResult`) (`self.LastImpactVelocity`)))
    (if _success
      (bind _returnvalue_3 (`self.GetNewSpeed` (`self.LastImpactResult`) _returnvalue_2 (`self.LastImpactVelocity`)))
      (if (> _returnvalue_3 0.0)
        (`self.Play_Hit_Effects` false _penetrationresult)
        (`MovementComponent.StopMovementImmediately` _prmovement)
        (clear `ProjectileMovementComponent.OnProjectileBounce` _prmovement)
        (`ActorComponent.K2_DestroyComponent` _prmovement)
        (`self.K2_SetActorLocation` _returnvalue_2 false true)
        (`self.ConstructProjectileMovement` (* _lastimpactvelocity (/ _returnvalue_3 (`KismetMathLibrary.VSize` _lastimpactvelocity))) (`self.BulletInitialSpeed`))
        (else
          (`MovementComponent.StopMovementImmediately` (`self.PRMovement`) :!label _label)
          (`self.Destroy_Projectile`)))
      (else
        (goto _label)))
    (else
      (`self.Play_Hit_Effects` true (`self.LastImpactResult`)))))

(event `self.FlyByChecker.OnComponentBeginOverlap`
  (params (OverlappedComponent :type "PrimitiveComponent Object Reference") (OtherActor :type "Actor Object Reference") (OtherComp :type "PrimitiveComponent Object Reference") (OtherBodyIndex :type Integer) (bFromSweep :type Boolean) (SweepResult :type "HitResult Structure (by ref)"))
  ;[1 1 1] Play Bullet Flyby Sound - WIP
  (if (and (== (`GameplayStatics.GetObjectClass` OtherActor) "/Game/UltimateShooterKit/Blueprints/BP_TFPCharacter.BP_TFPCharacter_C") (!= OtherActor (`self.GetOwner`)))
    (`GameplayStatics.PlaySoundAtLocation` "/Game/UltimateShooterKit/Sounds/Bullet/Cue_Bullet_Flyby.Cue_Bullet_Flyby" (`self.K2_GetActorLocation`) (struct) (`KismetMathLibrary.MapRangeClamped` (`KismetMathLibrary.Vector_Distance` (`self.K2_GetActorLocation` OtherActor) (`self.K2_GetActorLocation`)) 300.0 70.0 0.2 1.0) 1.0 0.0 "/Game/UltimateShooterKit/Sounds/SoundClassesAndMixes/BP_SoundAttenuation.BP_SoundAttenuation" "/Game/UltimateShooterKit/Sounds/SoundClassesAndMixes/BP_SoundConcurrency.BP_SoundConcurrency" (`self.GetOwner`))))

(event `Destroy_Projectile`
  ;[1 1 1] Request Destroy Projectile
  (`KismetSystemLibrary.Delay` 0.1)
  (`self.K2_DestroyActor`))

(fn `CalculateProjectileExitLocation`
  (params (HitResult :type "HitResult Structure") (ImpactVelocity :type "Vector Structure"))
  (returns (ReturnValue :type "Vector Structure") (Success :type Boolean) (PenetrationResult :type "HitResult Structure"))
  (locals (LocReturnLocation :type "Vector Structure") (LocResultFound :type Boolean))
  (bind _locreturnlocation (`local.LocReturnLocation`))
  (bind (_bblockinghit _binitialoverlap _time _distance _location _impactpoint _normal _impactnormal _physmat _hitactor) (`GameplayStatics.BreakHitResult` (`local.HitResult`)))
  (bind (_bblockinghit_2 _binitialoverlap_2 _time_2 _distance_2 _location_2) (`GameplayStatics.BreakHitResult` (`local.HitResult`)))
  (bind (_outhits _returnvalue) (`KismetSystemLibrary.SphereTraceMultiForObjects` (+ (* (`KismetMathLibrary.Normal` (`local.ImpactVelocity`)) 500.0) _location_2) _location_2 (`SphereComponent.SphereRadius` (`self.Sphere`)) (`|MakeArray` "ObjectTypeQuery1" "ObjectTypeQuery2" "ObjectTypeQuery3" "ObjectTypeQuery5" "ObjectTypeQuery6" "ObjectTypeQuery4" :!type "EObjectTypeQuery Enum")))
  (if _returnvalue
    (bind (_arrayindex _arrayelement) (`/Engine/EditorBlueprintResources/StandardMacros.ReverseForEachLoop` _outhits)
      (:`LoopBody`
        (bind (_bblockinghit_3 _binitialoverlap_3 _time_3 _distance_3 _location_3 _impactpoint_2 _normal_2 _impactnormal_2 _physmat_2 _hitactor_2) (`GameplayStatics.BreakHitResult` _arrayelement))
        (if (== _hitactor_2 _hitactor)
          (set `local.LocReturnLocation` (+ _location_3 (* _impactnormal_2 10.0)))
          (bind (_outhit _returnvalue_2) (`KismetSystemLibrary.SphereTraceSingle` (+ (`KismetMathLibrary.Normal` (`local.ImpactVelocity`)) _locreturnlocation) _locreturnlocation (`SphereComponent.SphereRadius` (`self.Sphere`)) "TraceTypeQuery1" false (`|MakeArray` _hitactor) "None" true (struct :`G` 0.081708 :`B` 1.0 :`A` 1.0) (struct :`R` 1.0 :`G` 0.690395 :`A` 1.0)))
          (if _returnvalue_2
            (bind (_returnvalue_3 _success _penetrationresult) (`self.CalculateProjectileExitLocation` _outhit (`local.ImpactVelocity`)))
            (return _returnvalue_3 _success _penetrationresult)
            (else
              (return (`local.LocReturnLocation`) true _arrayelement)))))
      (:`Completed`
        (return (0.0 0.0 0.0) false)))
    (else
      (return (0.0 0.0 0.0) false))))

(fn `ConstructProjectileMovement`
  (params (Velocity :type "Vector Structure") (InitialSpeed :type "Float (double-precision)"))
  (bind _returnvalue (`AddComponent|NODE_AddProjectileMovementComponent-3`))
  (bind _output_get (set `self.PRMovement` _returnvalue))
  (add `ProjectileMovementComponent.OnProjectileBounce` _output_get (`|CreateDelegate` :!event `On_Custom_PR_Bounced`))
  (set `MovementComponent.Velocity` (`local.Velocity`) (`self.PRMovement`))
  (set `ProjectileMovementComponent.InitialSpeed` (`local.InitialSpeed`) (`self.PRMovement`)))

(fn `FindAngleBetweenTwoVectors`
  (params (Vector1 :type "Vector Structure") (Vector2 :type "Vector Structure"))
  (returns (ReturnValue :type "Float (double-precision)"))
  (return (`KismetMathLibrary.DegAcos` (`KismetMathLibrary.Dot_VectorVector` (`KismetMathLibrary.Normal` Vector1) (`KismetMathLibrary.Normal` Vector2)))))

(fn `FindBulletPenetration`
  (params (SurfaceType :type "EPhysicalSurface Enum" :default "SurfaceType_Default"))
  (returns (ReturnValue :type "/Game/UltimateShooterKit/Blueprints/Data/Structures/WeaponStructures/Struct_AmmoPenetration Structure") (Success :type Boolean))
  (locals (LocReturn :type "/Game/UltimateShooterKit/Blueprints/Data/Structures/WeaponStructures/Struct_AmmoPenetration Structure") (LocFound :type Boolean))
  (bind ((`BulletPenetrationSetup_19_B3D875E646E1DCBAD7D654A4A093287C` _bulletpenetrationsetup)) (break `/Game/UltimateShooterKit/Blueprints/Data/Structures/WeaponStructures/Struct_AmmoMaster` (`self.AmmunitionInfo`)))
  (if (>= (`KismetArrayLibrary.Array_Length` _bulletpenetrationsetup) 1)
    (for _array_element _bulletpenetrationsetup
      (if (== (`.SurfaceType_3_6B2D362D469A9EDD57547D8A9FFED08A` (break `/Game/UltimateShooterKit/Blueprints/Data/Structures/WeaponStructures/Struct_AmmoPenetration` _array_element)) (`local.SurfaceType`))
        (set `local.LocReturn` _array_element)
        (break)
        (else
          (set `local.LocFound` false))))
    (else
      (set `local.LocFound` false)))
  (return (`local.LocReturn`) (`local.LocFound`)))

(fn `FindBulletSFX`
  (params (SurfaceType :type "EPhysicalSurface Enum" :default "SurfaceType_Default"))
  (returns (ReturnValue :type "/Game/UltimateShooterKit/Blueprints/Data/Structures/WeaponStructures/Struct_AmmoSFX Structure") (Success :type Boolean))
  (locals (LocReturn :type "/Game/UltimateShooterKit/Blueprints/Data/Structures/WeaponStructures/Struct_AmmoSFX Structure") (LocFound :type Boolean))
  (bind ((`BulletSFXSetup_15_951024654BC773F3443840A1127368D8` _bulletsfxsetup)) (break `/Game/UltimateShooterKit/Blueprints/Data/Structures/WeaponStructures/Struct_AmmoMaster` (`self.AmmunitionInfo`)))
  (if (>= (`KismetArrayLibrary.Array_Length` _bulletsfxsetup) 1)
    (for _array_element _bulletsfxsetup
      (if (== (`.SurfaceType_3_6B2D362D469A9EDD57547D8A9FFED08A` (break `/Game/UltimateShooterKit/Blueprints/Data/Structures/WeaponStructures/Struct_AmmoSFX` _array_element)) (`local.SurfaceType`))
        (set `local.LocReturn` _array_element)
        (break)
        (else
          (set `local.LocFound` false))))
    (else
      (set `local.LocFound` false)))
  (return (`local.LocReturn`) (`local.LocFound`)))

(fn `FindBulletVFX`
  (params (SurfaceType :type "EPhysicalSurface Enum" :default "SurfaceType_Default"))
  (returns (ReturnValue :type "/Game/UltimateShooterKit/Blueprints/Data/Structures/WeaponStructures/Struct_AmmoVFX Structure") (Success :type Boolean))
  (locals (LocReturn :type "/Game/UltimateShooterKit/Blueprints/Data/Structures/WeaponStructures/Struct_AmmoVFX Structure") (LocFound :type Boolean))
  (bind ((`BulletVFXSetup_16_C350BD9C4DBAEEDE06102D8788E9FCF3` _bulletvfxsetup)) (break `/Game/UltimateShooterKit/Blueprints/Data/Structures/WeaponStructures/Struct_AmmoMaster` (`self.AmmunitionInfo`)))
  (if (>= (`KismetArrayLibrary.Array_Length` _bulletvfxsetup) 1)
    (for _array_element _bulletvfxsetup
      (if (== (`.SurfaceType_3_6B2D362D469A9EDD57547D8A9FFED08A` (break `/Game/UltimateShooterKit/Blueprints/Data/Structures/WeaponStructures/Struct_AmmoVFX` _array_element)) (`local.SurfaceType`))
        (set `local.LocReturn` _array_element)
        (break)
        (else
          (set `local.LocFound` false))))
    (else
      (set `local.LocFound` false)))
  (return (`local.LocReturn`) (`local.LocFound`)))

(fn `FindTraceColor`
  (params (Velocity :type "Vector Structure"))
  (returns (ReturnValue :type "LinearColor Structure"))
  (bind _returnvalue (/ (`KismetMathLibrary.VSize` Velocity) (`ProjectileMovementComponent.InitialSpeed` (`self.PRMovement`))))
  (if (> _returnvalue 0.75)
    (return (`KismetMathLibrary.LinearColorLerp` (struct :`R` 1.0 :`G` 0.764 :`A` 1.0) (struct :`R` 1.0 :`A` 1.0) (* (- _returnvalue 0.75) 4.0)))
    (elif (> _returnvalue 0.5)
      (return (`KismetMathLibrary.LinearColorLerp` (struct :`G` 0.611765 :`A` 1.0) (struct :`R` 1.0 :`G` 0.764706 :`A` 1.0) (* (- _returnvalue 0.5) 4.0)))
      (elif (> _returnvalue 0.25)
        (return (`KismetMathLibrary.LinearColorLerp` (struct :`G` 0.446 :`B` 1.0 :`A` 1.0) (struct :`G` 0.611765 :`A` 1.0) (* (- _returnvalue 0.25) 4.0)))))))

(fn `GetNewSpeed`
  (params (HitResult :type "HitResult Structure") (ExitLocation :type "Vector Structure") (ImpactVelocity :type "Vector Structure"))
  (returns (ReturnValue :type "Float (double-precision)"))
  (locals (LocPenetrationData :type "/Game/UltimateShooterKit/Blueprints/Data/Structures/WeaponStructures/Struct_PenetrationData Structure"))
  (bind _returnvalue (/ (- (* 0.5 0.008 (`KismetMathLibrary.VSizeSquared` (`local.ImpactVelocity`))) (* (`KismetMathLibrary.VSize` (- (`local.ExitLocation`) (`.Location` (`GameplayStatics.BreakHitResult` (`local.HitResult`))))) (`.EnergyToSubtract_17_A0D54D744A583584D76BC4B5BB2A8AE8` (break `/Game/UltimateShooterKit/Blueprints/Data/Structures/WeaponStructures/Struct_PenetrationData` (`local.LocPenetrationData`))) 10.0)) (* 0.5 0.008)))
  ;[1 1 1] Get Penetration Data Depends On The Surface
  (set `local.LocPenetrationData` (`.PenetrationSetup_20_7BDA651A484BD6B28B566DB7F05F5275` (break `/Game/UltimateShooterKit/Blueprints/Data/Structures/WeaponStructures/Struct_AmmoPenetration` (`self.FindBulletPenetration` (`GameplayStatics.GetSurfaceType` (`local.HitResult`))))))
  (if (>= _returnvalue 0.0)
    (return (`KismetMathLibrary.Sqrt` _returnvalue))
    (else
      (return 0.0))))

(fn `ShouldPenetrate`
  (params (HitResult :type "HitResult Structure") (ImpactVelocity :type "Vector Structure"))
  (returns (ReturnValue :type Boolean))
  (locals (LocBounced :type Boolean :default false))
  (bind ((`ChanceOfBounce_26_74AE88924041573C8F16AABCEA075AA2` _chanceofbounce) (`MinAngleForBounce_22_A76598DA42905F9A1558E4B9B144BEFB` _minangleforbounce)) (break `/Game/UltimateShooterKit/Blueprints/Data/Structures/WeaponStructures/Struct_PenetrationData` (`.PenetrationSetup_20_7BDA651A484BD6B28B566DB7F05F5275` (break `/Game/UltimateShooterKit/Blueprints/Data/Structures/WeaponStructures/Struct_AmmoPenetration` (`self.FindBulletPenetration` (`GameplayStatics.GetSurfaceType` (`local.HitResult`)))))))
  ;[1 1 1] Decide If The Bullet Should Penetrate Or Not
  (bind _returnvalue (`self.FindAngleBetweenTwoVectors` (`local.ImpactVelocity`) (* (`.ImpactNormal` (`GameplayStatics.BreakHitResult` (`local.HitResult`))) -1.0)))
  (set `local.LocBounced` (`KismetMathLibrary.RandomBoolWithWeight` _chanceofbounce))
  (return (select `bool` (> _returnvalue _minangleforbounce) :`false` true :`true` (not (`local.LocBounced`)))))

(fn `UpdateHitVars`
  (params (Hit :type "HitResult Structure (by ref)"))
  (bind (_bblockinghit _binitialoverlap _time _distance _location _impactpoint _normal) (`GameplayStatics.BreakHitResult` Hit))
  (set `self.LastHitSurfaceType` (`GameplayStatics.GetSurfaceType` Hit))
  (set `self.LastHitTransform` (`KismetMathLibrary.MakeTransform` _location (`KismetMathLibrary.Conv_VectorToRotator` _normal)))
  (set `self.MirroredRotation` (`KismetMathLibrary.Conv_VectorToRotator` (`KismetMathLibrary.MirrorVectorByNormal` (`self.BulletDirection`) _normal))))

(fn `UserConstructionScript`)