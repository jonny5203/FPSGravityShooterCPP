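; Game State for the Capture the Flag mode that keeps both teams' scores and detects the winner.
; AddTeamPoints takes a boolean team flag, true for Team B and false for Team A, and increments that team's points.
; When a score reaches PointsToWin, it casts the game mode to BP_Base_GM and calls ServerEndGame with the winning team's flag.
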(event `AddTeamPoints`
  (params (bTeam :type Boolean))
  (if bTeam
    (bind _result (`/Engine/EditorBlueprintResources/StandardMacros.IncrementInt` (`self.TeamBPoints`))
      (:`  `
        (bind _output_get (set `self.TeamBPoints` _result))
        (if (>= _output_get (`self.PointsToWin`))
          (bind _asbp_base_gm (cast `/Game/FPS/Blueprints/GameModes/BP_Base_GM` (`GameplayStatics.GetGameMode`)))
          (`/Game/FPS/Blueprints/GameModes/BP_Base_GM.Server_EndGame` _asbp_base_gm true))))
    (else
      (bind _result_2 (`/Engine/EditorBlueprintResources/StandardMacros.IncrementInt` (`self.TeamAPoints`))
        (:`  `
          (bind _output_get_2 (set `self.TeamAPoints` _result_2))
          (if (>= _output_get_2 (`self.PointsToWin`))
            (bind _asbp_base_gm_2 (cast `/Game/FPS/Blueprints/GameModes/BP_Base_GM` (`GameplayStatics.GetGameMode`)))
            (`/Game/FPS/Blueprints/GameModes/BP_Base_GM.Server_EndGame` _asbp_base_gm_2 false)))))))

(fn `UserConstructionScript`
  (`parent.UserConstructionScript`))