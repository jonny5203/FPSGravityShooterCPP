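; BP_Lobby_GS is the lobby game state that runs the countdown before the game launches.
; StartCountDown runs only on the authority, flags the countdown active and starts a one-shot timer that calls ServerLaunchGame on BP_Lobby_GM when it expires.
; A faster looping timer copies the countdown timer's remaining time into TimeLeftCountDown.
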(event `StartCountDown`
  ;[1 1 1] CountDown
  (`/Engine/EditorBlueprintResources/ActorMacros.Switch Has Authority`
    (:`Authority`
      (bind _returnvalue (`KismetSystemLibrary.K2_SetTimerDelegate` (delegate `LaunchMap`) 30.0))
      (set `self.CountDownHandle` _returnvalue)
      (set `self.bIsCountDownActive` true)
      (`KismetSystemLibrary.K2_SetTimerDelegate` (delegate `UpdateTimeLeft`) 0.1 true))))

(event `LaunchMap`
  ;[1 1 1] CountDown
  (bind _asbp_lobby_gm (cast `/Game/FPS/Blueprints/GameModes/Lobby/BP_Lobby_GM` (`GameplayStatics.GetGameMode`)))
  (`/Game/FPS/Blueprints/GameModes/Lobby/BP_Lobby_GM.Server_LaunchGame` _asbp_lobby_gm))

(event `UpdateTimeLeft`
  ;[1 1 1] CountDown
  (set `self.TimeLeftCountDown` (`KismetSystemLibrary.K2_GetTimerRemainingTimeHandle` (`self.CountDownHandle`))))

(fn `UserConstructionScript`)