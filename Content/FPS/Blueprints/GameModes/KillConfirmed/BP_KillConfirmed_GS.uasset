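; Game state for the Kill Confirmed mode that tracks both teams' scores and the dogtags in play.
; Server_AddTeamPoints increments the score of the team picked by a boolean and, at PointsToWin, tells the BP_Base_GM game mode to end the match with that winner.
; A unique-entry dogtag array supports registering tags, removing and destroying them, and refreshing the material on every valid tag.
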(event `Server_AddTeamPoints`
  (params (bTeam :type Boolean))
  ;[1 1 1] Add Points on kill
  (if bTeam
    (bind _result (`/Engine/EditorBlueprintResources/StandardMacros.IncrementInt` (`self.TeamB_Points`))
      (:`  `
        (bind _output_get (set `self.TeamB_Points` _result))
        (if (>= _output_get (`self.PointsToWin`))
          (bind _asbp_base_gm (cast `/Game/FPS/Blueprints/GameModes/BP_Base_GM` (`GameplayStatics.GetGameMode`)))
          (`/Game/FPS/Blueprints/GameModes/BP_Base_GM.Server_EndGame` _asbp_base_gm true))))
    (else
      (bind _result_2 (`/Engine/EditorBlueprintResources/StandardMacros.IncrementInt` (`self.TeamA_Points`))
        (:`  `
          (bind _output_get_2 (set `self.TeamA_Points` _result_2))
          (if (>= _output_get_2 (`self.PointsToWin`))
            (bind _asbp_base_gm_2 (cast `/Game/FPS/Blueprints/GameModes/BP_Base_GM` (`GameplayStatics.GetGameMode`)))
            (`/Game/FPS/Blueprints/GameModes/BP_Base_GM.Server_EndGame` _asbp_base_gm_2 false)))))))

(event `UpdateDogtagsMaterial`
  (bind _dogtags (`self.Dogtags`))
  ;[1 1 1] Update Dogtags Material
  (if (`KismetArrayLibrary.Array_IsValidIndex` _dogtags)
    (for _array_element _dogtags
      (`/Engine/EditorBlueprintResources/StandardMacros.IsValid` _array_element
        (:`Is Valid`
          (`/Game/FPS/Blueprints/GameObjectives/KillConfirmDogTag/BP_DogTag.UpdateMaterial` _array_element))))))

(event `AddNewDogtag`
  (params (NewDogtag :type "/Game/FPS/Blueprints/GameObjectives/KillConfirmDogTag/BP_DogTag Object Reference"))
  ;[1 1 1] Add New Dogtag
  (`KismetArrayLibrary.Array_AddUnique` (`self.Dogtags`) NewDogtag))

(event `RemoveDogTag`
  (params (DogtagToDelete :type "/Game/FPS/Blueprints/GameObjectives/KillConfirmDogTag/BP_DogTag Object Reference"))
  ;[1 1 1] RemoveDogtag
  (`KismetArrayLibrary.Array_RemoveItem` (`self.Dogtags`) DogtagToDelete)
  (`self.K2_DestroyActor` DogtagToDelete))

(fn `UserConstructionScript`)