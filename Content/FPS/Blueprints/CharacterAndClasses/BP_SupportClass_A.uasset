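; Support class character whose skill places a mine in front of the player.
; UseClassSkill checks the cooldown flag, plays a sound and traces forward and down from the actor to find the placement point.
; ServerSpawnMine then spawns BP_Mine there, recording the controller as instigator.
; A timer re-enables the skill after the cooldown, with the gameplay widget notified on use and reset.
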(event `ResetSkill`
  ;[1 1 1] Reset Skill
  (set `self.bCanUseSkill` true)
  (`/Game/FPS/UI/Gameplay/WB_Gameplay.SkillReset` (`/Game/FPS/Blueprints/PlayerController/BP_BasePlayerController.GameplayWBRef` (`self.ControllerRef`))))

(event `self.UseClassSkill`
  (bind _returnvalue (`self.K2_GetActorLocation`))
  ;[0.6685 0.7443 1] Class Skill
  (if (`self.bCanUseSkill`)
    (set `self.bCanUseSkill` false)
    (bind _returnvalue_2 (`KismetSystemLibrary.K2_SetTimerDelegate` (delegate `ResetSkill`) (`self.AbilityCoolDown`)))
    (`/Game/FPS/UI/Gameplay/WB_Gameplay.OnSkillUsed` (`/Game/FPS/Blueprints/PlayerController/BP_BasePlayerController.GameplayWBRef` (`self.ControllerRef`)) _returnvalue_2)
    (`GameplayStatics.PlaySound2D` "/Engine/VREditor/Sounds/UI/Object_PickUp.Object_PickUp" 1.0 1.0 0.0 null null)
    (bind _outhit (`KismetSystemLibrary.LineTraceSingle` _returnvalue (+ _returnvalue (+ (* (`self.GetActorForwardVector`) 1000.0) (* (`self.GetActorUpVector`) -500.0))) "TraceTypeQuery1"))
    (`self.ServerSpawnMine` (`KismetMathLibrary.Conv_VectorToTransform` (`.Location` (`GameplayStatics.BreakHitResult` _outhit))))))

(event `ServerSpawnMine`
  (params (NewParam :type "Transform Structure"))
  ;[0.6685 0.7443 1] Class Skill
  (bind _returnvalue (`|SpawnActorFromClass` "/Game/FPS/Blueprints/Mine/BP_Mine.BP_Mine_C" NewParam "Undefined" "OverrideRootScale" self self))
  (set `/Game/FPS/Blueprints/Mine/BP_Mine.ControllerInstigator` (`self.GetController`) _returnvalue))

(fn `UserConstructionScript`
  (`parent.UserConstructionScript`))