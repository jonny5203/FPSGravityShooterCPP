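; Spawn protection zone for the FPS mode that warns enemy players who enter a team's spawn area.
; Box overlap events compare the entering or leaving character's PlayerState team against SpawnTeam, toggling the warning on BP_BaseCharacter for non-matching teams.
; The construction script sizes the box from BoxX and BoxY with a fixed height.
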(event `self.Box.OnComponentBeginOverlap`
  (params (OverlappedComponent :type "PrimitiveComponent Object Reference") (OtherActor :type "Actor Object Reference") (OtherComp :type "PrimitiveComponent Object Reference") (OtherBodyIndex :type Integer) (bFromSweep :type Boolean) (SweepResult :type "HitResult Structure (by ref)"))
  (bind _asbp_base_character (cast `/Game/FPS/Blueprints/CharacterAndClasses/BP_BaseCharacter` OtherActor))
  (bind _asbp_player_state (cast `/Game/FPS/Blueprints/GameModes/BP_PlayerState` (`Pawn.PlayerState` _asbp_base_character)))
  (if (not (== (`/Game/FPS/Blueprints/GameModes/BP_PlayerState.Team` _asbp_player_state) (`self.SpawnTeam`)))
    (`/Game/FPS/Blueprints/CharacterAndClasses/BP_BaseCharacter.SetWarnPlayer` _asbp_base_character true)))

(event `self.Box.OnComponentEndOverlap`
  (params (OverlappedComponent :type "PrimitiveComponent Object Reference") (OtherActor :type "Actor Object Reference") (OtherComp :type "PrimitiveComponent Object Reference") (OtherBodyIndex :type Integer))
  (bind _asbp_base_character (cast `/Game/FPS/Blueprints/CharacterAndClasses/BP_BaseCharacter` OtherActor))
  (bind _asbp_player_state (cast `/Game/FPS/Blueprints/GameModes/BP_PlayerState` (`Pawn.PlayerState` _asbp_base_character)))
  (if (not (== (`/Game/FPS/Blueprints/GameModes/BP_PlayerState.Team` _asbp_player_state) (`self.SpawnTeam`)))
    (`/Game/FPS/Blueprints/CharacterAndClasses/BP_BaseCharacter.SetWarnPlayer` _asbp_base_character false)))

(fn `UserConstructionScript`
  (`BoxComponent.SetBoxExtent` (`self.Box`) (`KismetMathLibrary.MakeVector` (`self.Box_X`) (`self.Box_Y`) 300.0) true))