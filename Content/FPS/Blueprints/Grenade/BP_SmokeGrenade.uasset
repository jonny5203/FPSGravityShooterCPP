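; BP_SmokeGrenade is a smoke grenade that, when exploded on the server, emits a particle effect for a fixed duration.
; ServerExplodeGrenade sets a replicated smoke-active flag once, forces a net update, then destroys the actor after a delay.
; The flag's RepNotify spawns the emitter attached to the Sphere component, so the visuals follow replicated state rather than a separate effect RPC.
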(event `self.Server_ExplodeGrenade`
  (if (not (`self.bIsSmokeActive`))
    (set `self.bIsSmokeActive` true)
    (`self.ForceNetUpdate`)
    (`KismetSystemLibrary.Delay` 30.0)
    (`self.K2_DestroyActor`)))

(fn `OnRep_bIsSmokeActive`
  (bind _sphere (`self.Sphere`))
  (if (`self.bIsSmokeActive`)
    (`GameplayStatics.SpawnEmitterAttached` "/Game/FPS/Effects/Particles/Snow/P_BlowDetails.P_BlowDetails" _sphere "None" (`SceneComponent.K2_GetComponentLocation` _sphere) (struct) (1.0 1.0 1.0) "KeepWorldPosition")))

(fn `UserConstructionScript`
  (`parent.UserConstructionScript`))