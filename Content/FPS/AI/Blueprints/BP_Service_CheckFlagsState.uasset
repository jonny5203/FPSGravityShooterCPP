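; Behavior tree service that keeps an AI bot's blackboard updated on the state of the flags in the level.
; On each AI tick it gathers every BP_BaseFlag actor and compares its team to the controlled character's PawnTeam.
; Each flag's FlagTaken state is written to TeamFlagTaken for a matching team, otherwise to EnemyFlagTaken.
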(event `self.ReceiveTickAI`
  (params (OwnerController :type "AIController Object Reference") (ControlledPawn :type "Pawn Object Reference") (DeltaSeconds :type "Float (single-precision)"))
  (bind _outactors (`GameplayStatics.GetAllActorsOfClass` "/Game/FPS/Blueprints/GameObjectives/CTF_Flag/BP_BaseFlag.BP_BaseFlag_C"))
  (for _array_element _outactors
    (if (== (`/Game/FPS/Blueprints/GameObjectives/CTF_Flag/BP_BaseFlag.Team` _array_element) (`/Game/FPS/Blueprints/CharacterAndClasses/BP_BaseCharacter.bPawnTeam` (cast `/Game/FPS/Blueprints/CharacterAndClasses/BP_BaseCharacter` ControlledPawn :!pure true)))
      (bind _bflagtaken (`/Game/FPS/Blueprints/GameObjectives/CTF_Flag/BP_BaseFlag.bFlagTaken` _array_element))
      (`BTFunctionLibrary.SetBlackboardValueAsBool` (`self.TeamFlagTaken`) _bflagtaken)
      (else
        (`BTFunctionLibrary.SetBlackboardValueAsBool` (`self.EnemyFlagTaken`) _bflagtaken)))))