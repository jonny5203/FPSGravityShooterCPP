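; Behavior Tree service that writes the location of a random enemy character to a vector Blackboard key on each AI tick.
; It gathers BP_BaseCharacter pawns from the GameState's PlayerArray, then FindEnemies keeps those on a different PawnTeam than the controlled pawn.
; The random index is re-rolled between the validity check and the location read, so the two can hit different enemies.
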(event `self.ReceiveTickAI`
  (params (OwnerController :type "AIController Object Reference") (ControlledPawn :type "Pawn Object Reference") (DeltaSeconds :type "Float (single-precision)"))
  (`KismetArrayLibrary.Array_Clear` (`self.PosibleEnemies`))
  (bind _asbp_base_gs (cast `/Game/FPS/Blueprints/GameModes/BP_Base_GS` (`GameplayStatics.GetGameState`)))
  (for _array_element (`GameStateBase.PlayerArray` _asbp_base_gs)
    (bind _asbp_base_character (cast `/Game/FPS/Blueprints/CharacterAndClasses/BP_BaseCharacter` (`PlayerState.PawnPrivate` _array_element)))
    (`KismetArrayLibrary.Array_AddUnique` (`self.PosibleEnemies`) _asbp_base_character))
  (bind _enemies (`self.FindEnemies` ControlledPawn (`self.PosibleEnemies`)))
  (if (`KismetArrayLibrary.Array_IsValidIndex` _enemies)
    (bind _output (`|GetArrayItem` _enemies (`KismetMathLibrary.RandomIntegerInRange` 0 (`KismetArrayLibrary.Array_LastIndex` _enemies))))
    (`/Engine/EditorBlueprintResources/StandardMacros.IsValid` _output
      (:`Is Valid`
        (`BTFunctionLibrary.SetBlackboardValueAsVector` (`self.Vectorkey`) (`Actor.K2_GetActorLocation` _output))))))

(fn `FindEnemies`
  (params (SelfPawn :type "Pawn Object Reference") (PossibleEnemies :type "Array of /Game/FPS/Blueprints/CharacterAndClasses/BP_BaseCharacter Object Reference"))
  (returns (Enemies :type "Array of /Game/FPS/Blueprints/CharacterAndClasses/BP_BaseCharacter Object Reference"))
  (locals (EnemiesArray :type "Array of /Game/FPS/Blueprints/CharacterAndClasses/BP_BaseCharacter Object Reference"))
  (bind _asbp_base_character (cast `/Game/FPS/Blueprints/CharacterAndClasses/BP_BaseCharacter` SelfPawn :!pure true))
  (`KismetArrayLibrary.Array_Clear` (`local.EnemiesArray`))
  (for _array_element PossibleEnemies
    (if (and (!= _array_element _asbp_base_character) (!= (`/Game/FPS/Blueprints/CharacterAndClasses/BP_BaseCharacter.bPawnTeam` _array_element) (`/Game/FPS/Blueprints/CharacterAndClasses/BP_BaseCharacter.bPawnTeam` _asbp_base_character)))
      (`KismetArrayLibrary.Array_AddUnique` (`local.EnemiesArray`) _array_element)))
  (return (`local.EnemiesArray`)))