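; Behavior tree service that picks an enemy for an AI pawn and writes it to the blackboard.
; Each tick it filters sight-perceived characters to living opponents on other teams, storing the chosen one and its location, or clearing the enemy key when none qualify.
; FindClosestEnemy measures the current pick rather than each candidate, so the result is not reliably the nearest.
; IsEnemyAlive, which clears dead targets, is not called here.
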(event `self.ReceiveTickAI`
  (params (OwnerController :type "AIController Object Reference") (ControlledPawn :type "Pawn Object Reference") (DeltaSeconds :type "Float (single-precision)"))
  (`KismetArrayLibrary.Array_Clear` (`self.PosibleEnemies`))
  (for _array_element (`AIPerceptionComponent.GetKnownPerceivedActors` (`Actor.GetComponentByClass` OwnerController "/Script/AIModule.AIPerceptionComponent") "/Script/AIModule.AISense_Sight")
    (bind _asbp_base_character (cast `/Game/FPS/Blueprints/CharacterAndClasses/BP_BaseCharacter` _array_element))
    (if (and (not (`/Game/FPS/Blueprints/CharacterAndClasses/BP_BaseCharacter.bDead` _asbp_base_character)) (!= (`/Game/FPS/Blueprints/CharacterAndClasses/BP_BaseCharacter.bPawnTeam` _asbp_base_character) (`/Game/FPS/Blueprints/CharacterAndClasses/BP_BaseCharacter.bPawnTeam` (cast `/Game/FPS/Blueprints/CharacterAndClasses/BP_BaseCharacter` ControlledPawn :!pure true))))
      (`KismetArrayLibrary.Array_Add` (`self.PosibleEnemies`) _asbp_base_character)))
  (if (`KismetArrayLibrary.Array_IsValidIndex` (`self.PosibleEnemies`))
    (bind _enemy (`self.FindClosestEnemy` (`self.PosibleEnemies`) ControlledPawn))
    (`/Engine/EditorBlueprintResources/StandardMacros.IsValid` _enemy
      (:`Is Valid`
        (`BTFunctionLibrary.SetBlackboardValueAsVector` (`self.Vectorkey`) (`Actor.K2_GetActorLocation` _enemy))
        (`BTFunctionLibrary.SetBlackboardValueAsObject` (`self.EnemyKey`) _enemy)))
    (else
      (`BTFunctionLibrary.SetBlackboardValueAsObject` (`self.EnemyKey`)))))

(fn `FindClosestEnemy`
  (params (Enemys :type "Array of /Game/FPS/Blueprints/CharacterAndClasses/BP_BaseCharacter Object Reference") (SelfPawn :type "Pawn Object Reference"))
  (returns (Enemy :type "/Game/FPS/Blueprints/CharacterAndClasses/BP_BaseCharacter Object Reference"))
  (locals (MinDistance :type "Float (double-precision)" :default 2500000.0))
  (bind _enemy (`self.Enemy`))
  (bind _returnvalue (`KismetMathLibrary.Abs` (`KismetMathLibrary.VSize` (- (`Actor.K2_GetActorLocation` _enemy) (`Actor.K2_GetActorLocation` SelfPawn)))))
  (set `local.MinDistance` 250000.0)
  (for _array_element Enemys
    (`/Engine/EditorBlueprintResources/StandardMacros.IsValid` _enemy
      (:`Is Valid`
        (if (< _returnvalue (`local.MinDistance`))
          (set `self.Enemy` _array_element)
          (set `local.MinDistance` _returnvalue)))
      (:`Is Not Valid`
        (set `self.Enemy` _array_element))))
  (return (`self.Enemy`)))

(fn `IsEnemyAlive`
  (params (Enemy :type "/Game/FPS/Blueprints/CharacterAndClasses/BP_BaseCharacter Object Reference"))
  (if (`/Game/FPS/Blueprints/CharacterAndClasses/BP_BaseCharacter.bDead` Enemy)
    (`BTFunctionLibrary.SetBlackboardValueAsObject` (`self.EnemyKey`))))