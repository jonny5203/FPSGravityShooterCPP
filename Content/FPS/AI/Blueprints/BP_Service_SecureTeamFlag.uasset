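; Behavior tree service for flag-game AI that writes a target location to a blackboard vector key on each service tick.
; If the controlled pawn carries a flag, the target is its own team flag's initial position.
; Otherwise it targets the location of a flag-carrying teammate, leaving the key untouched if none exists.
; Flags and characters are found with GetAllActorsOfClass scans and matched by team.
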(event `self.ReceiveTickAI`
  (params (OwnerController :type "AIController Object Reference") (ControlledPawn :type "Pawn Object Reference") (DeltaSeconds :type "Float (single-precision)"))
  (bind _asbp_base_character (cast `/Game/FPS/Blueprints/CharacterAndClasses/BP_BaseCharacter` ControlledPawn :!pure true))
  (bind _outactors (`GameplayStatics.GetAllActorsOfClass` "/Game/FPS/Blueprints/GameObjectives/CTF_Flag/BP_BaseFlag.BP_BaseFlag_C"))
  (for _array_element _outactors
    (if (== (`/Game/FPS/Blueprints/GameObjectives/CTF_Flag/BP_BaseFlag.Team` _array_element) (`/Game/FPS/Blueprints/CharacterAndClasses/BP_BaseCharacter.bPawnTeam` _asbp_base_character))
      (if (`/Game/FPS/Blueprints/CharacterAndClasses/BP_BaseCharacter.bCarringFlag` _asbp_base_character)
        (`BTFunctionLibrary.SetBlackboardValueAsVector` (`self.Vectorkey`) (`/Game/FPS/Blueprints/GameObjectives/CTF_Flag/BP_BaseFlag.InitialPossition` _array_element))
        (else
          (bind _outactors_2 (`GameplayStatics.GetAllActorsOfClass` "/Game/FPS/Blueprints/CharacterAndClasses/BP_BaseCharacter.BP_BaseCharacter_C"))
          (for _array_element_2 _outactors_2
            (if (and (`/Game/FPS/Blueprints/CharacterAndClasses/BP_BaseCharacter.bCarringFlag` _array_element_2) (== (`/Game/FPS/Blueprints/CharacterAndClasses/BP_BaseCharacter.bPawnTeam` _array_element_2) (`/Game/FPS/Blueprints/CharacterAndClasses/BP_BaseCharacter.bPawnTeam` _asbp_base_character)))
              (`BTFunctionLibrary.SetBlackboardValueAsVector` (`self.Vectorkey`) (`Actor.K2_GetActorLocation` _array_element_2)))))))))