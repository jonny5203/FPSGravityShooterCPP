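; Behavior tree service that tracks an enemy flag carrier for AI characters in a flag-carrying FPS mode.
; On each AI tick it scans every BP_BaseCharacter for one carrying a flag on a different team from the controlled pawn.
; It writes that carrier's position to the Location blackboard key; the last match wins, and the key is left unchanged when none is found.
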(event `self.ReceiveTickAI`
  (params (OwnerController :type "AIController Object Reference") (ControlledPawn :type "Pawn Object Reference") (DeltaSeconds :type "Float (single-precision)"))
  (bind _outactors (`GameplayStatics.GetAllActorsOfClass` "/Game/FPS/Blueprints/CharacterAndClasses/BP_BaseCharacter.BP_BaseCharacter_C"))
  (for _array_element _outactors
    (if (and (`/Game/FPS/Blueprints/CharacterAndClasses/BP_BaseCharacter.bCarringFlag` _array_element) (!= (`/Game/FPS/Blueprints/CharacterAndClasses/BP_BaseCharacter.bPawnTeam` _array_element) (`/Game/FPS/Blueprints/CharacterAndClasses/BP_BaseCharacter.bPawnTeam` (cast `/Game/FPS/Blueprints/CharacterAndClasses/BP_BaseCharacter` ControlledPawn :!pure true))))
      (`BTFunctionLibrary.SetBlackboardValueAsVector` (`self.Location`) (`Actor.K2_GetActorLocation` _array_element)))))